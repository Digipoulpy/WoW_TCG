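; Player controller for a networked trading card game, handling the client side of card play, turns and match flow.
; Drag-drop stores pending card data during the player's turn; placement and interaction logic validates locally before requesting server execution, with failed drops logged.
; Server-facing events return the saved deck, set the countdown and end the match.
; After login it builds player and opponent UI, refreshed with health and turn state.
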(event Custom|4.14_OnDragCanceled
  ;[0 0 0] Input Events - Card Placement and Interaction
)

(event Custom|Event_GetPlayerDeck
  ;[0 0 0] Version 1.1 - Called by the server to get and load the players chosen deck
  (bind (_deckname _deck) (CallFunction|LoadClientDeck))
  (CallFunction|ServerReturnPlayerDeck _deckname _deck))

(event Custom|ClientPostLogin
  ;[0 0 0] Client Post Login - Handles the inital game setup of the players deck, Game UI and player respawn
  (Utilities|FlowControl|Delay 1.0) ; This short delay helps stop referencing actors that might not yet be available.
  (bind _astcg_game_instance (Utilities|Casting|CastToTCG_GameInstance (Game|GetGameInstance)))
  (if (.In%20State%20 (Default|GetGameState _astcg_game_instance "NewEnumerator0")) ; Is game currently in "Playing" state?
    (CallFunction|SetupGameUI)
    (CallFunction|UpdateGameUI false)))

(event Custom|LogNotificationMessage
  (params (Message :type String) (Colour :type Linear%20Color%20Structure))
  ;[0 0 0] OwningClient - Create Display Message
)

(event Custom|DestroyClientCard
  ;[0 0 0] Play Card - Drop and Play Card (Step 3)
  (Actor|DestroyActor (Variables|Default|GetPlayCard_Client_Ref))
  (Variables|Default|SetPlayCard_Client_Ref 0))

(event Custom|SpawnAIOpponent
  (Utilities|Casting|CastTo (Game|GetGameMode)))

(event Custom|Call%20Create%20Card
  (params (Card%20Name :type Name) (DragDrop%20Operation :type Drag%20Drop%20Operation%20Object%20Reference) (CardSet :type Byte) (CardHandIndex :type Integer))
  ;[0 0 0] Create a client side card visual for the player to determin where to place the card. Note: This does not create the serverside card, it only sets the variables and client state until the card is played.
  (if (Variables|Default|GetbTurnActive) ; Check Added Version 1.1
    (Variables|Default|SetDragDrop%20Operation%20Ref DragDrop%20Operation)
    (bind _output_get (Variables|Default|SetTemp_CreateCardName Card%20Name))
    (bind _output_get_2 (Variables|Default|SetTemp_ChosenCardSet CardSet))
    (Variables|Default|SetTempHandIndex CardHandIndex)))

(event Custom|UpdateGameUI
  (params (ForceCleanUpdate :type Boolean))
  (bind _playergameui_ref (Variables|Default|GetPlayerGameUI_Ref))
  ;[0 0 0] Update Game UI
  (Utilities|IsValid (Variables|Default|GetPlayerGameUI_Ref)
    (:Is%20Valid
      (CallFunction|ServerUpdatePlayerHealth)
      (Class|Object|UpdateUIPlayerStats(Message) (Variables|Default|GetOpponentUI_Ref) ForceCleanUpdate)
      (Class|Object|UpdateUIPlayerStats(Message) _playergameui_ref false)
      (Class|Object|UpdateUITurnState(Message) _playergameui_ref (Variables|Default|GetbTurnActive) (Variables|Default|GetTurnState)))))

(event Custom|Event_DropCard
  (params (CardPlayed :type Boolean) (Errors :type Byte))
  ;[0 0 0] Owning Client- Recieve the server result and update the client state when the card was either placed or if it was invalid
  (bind _output_get (Variables|Default|SetbIsPlayed CardPlayed))
  (if (not _output_get)
    (CallFunction|EventCreateDisplayMessage (Utilities|String|Append "DEBUG: " (Utilities|String|EnumtoString Errors)) "(R=1.000000,G=1.000000,B=1.000000,A=1.000000)" false 0.0 true)
    (Utilities|Casting|CastTo (Variables|/Script/UMG.DragDropOperation|GetPayload (Variables|Default|GetDragDrop%20Operation%20Ref)))))

(event Custom|Event_CreateDisplayMessage
  (params (Message :type String) (Specified%20Color :type Linear%20Color%20Structure) (ToScreen :type Boolean) (ScreenDuration :type Float%20%28single-precision%29) (ToMessageLogger :type Boolean))
  ;[0 0 0] OwningClient - Create Display Message
  (if (not ToScreen)
    (if ToMessageLogger
      _)))

(event Custom|SetCountdownTimer
  (params (Time :type Integer))
  ;[0 0 0] Set Countdown Timer
  (GameSetup|SetTimer Time))

(event Custom|Event_EndClientMatchState
  (params (NewParam :type Byte))
  ;[0 0 0] Event End Game - Set clients end game state
  (Default|SetCardViewState (Variables|/Game/WoW_TCG/Blueprints/Widgets/Player_Game_UI.Player_Game_UI_C|GetCard%20Manager (Variables|Player|GetPlayer%20Game%20UI%20Ref)) "NewEnumerator3" false))

(event EventBeginPlay
  ;[0 0 0] Event Begin Play - Set References to Game Mode, Game State and Player State
  (Input|SetInputModeGameandUI self 0 "DoNotLock" false)
  (Utilities|FlowControl|Delay 2.0)
  (bind _astcg_game_state (Utilities|Casting|CastToTCG_GameState (Game|GetGameState)))
  (Variables|System|SetGame%20State%20Ref _astcg_game_state)
  (bind _astcg_player_state (Utilities|Casting|CastToTCG_PlayerState (Variables|GetPlayerState self)))
  (Variables|System|SetPlayer%20State%20Ref _astcg_player_state))

(event EventMatchEnd
  (params (Results :type EndGameResults_Variable%20Enum :default "NewEnumerator0"))
  ;[0 0 0] Event End Game - Set clients end game state
  (Utilities|FlowControl|DoOnce false
    (:Completed
      (if (Variables|Player|GetTurn%20Active)
        (Variables|Player|SetTurn%20Active false))
      (Utilities|FlowControl|Delay 0.5)
      (CallFunction|EventEndClientMatchState Results))))

(event Input|MouseEvents|LeftMouseButton
  (params (Key :type Key%20Structure))
  ;[0 0 0] Input Events - Card Placement and Interaction
)

(event Input|TouchEvents|InputTouch
  (params (Location :type Vector) (FingerIndex :type ETouchIndex%20Enum))
  ;[0 0 0] Input Events - Card Placement and Interaction
)

(fn ConstructionScript)

(fn OnRepTurnActive)

(fn OnRepTurnState)

(fn SetupGameUI
  (if (Pawn|IsLocalPlayerController)
    ;[0.3255 1 0.2824 0.298] Add player UI
    (bind _returnvalue (UserInterface|CreateWidget "/Game/WoW_TCG/Blueprints/Widgets/Player_Game_UI.Player_Game_UI_C" self))
    (bind _output_get (Variables|Player|SetPlayer%20Game%20UI%20Ref _returnvalue))
    (UserInterface|Viewport|AddtoViewport _output_get 2)
    ;[0.3255 1 0.2824 0.298] Add Opponent UI
    (bind _returnvalue_2 (UserInterface|CreateWidget "/Game/WoW_TCG/Blueprints/Widgets/Opponent_UI.Opponent_UI_C" self))
    (bind _output_get_2 (Variables|Player|SetOpponent%20UI%20Ref _returnvalue_2))
    (UserInterface|Viewport|AddtoViewport _output_get_2 1))
  (return))

(fn SetTimer
  (params (Time :type Integer))
  (Utilities|IsValid (Variables|Game|GetCountdown%20Timer%20Widget)
    (:Is%20Valid
      (bind _output_get (Variables|/Game/WoW_TCG/Blueprints/Widgets/Countdown_Timer.Countdown_Timer_C|SetTimer (stale _output_get_2) Time))
      (if (< _output_get 1)
        (Widget|RemovefromParent (Variables|Game|GetCountdown%20Timer%20Widget))))
    (:Is%20Not%20Valid
      (bind _returnvalue (UserInterface|CreateWidget "/Game/WoW_TCG/Blueprints/Widgets/Countdown_Timer.Countdown_Timer_C" self))
      (bind _output_get_2 (Variables|Game|SetCountdown%20Timer%20Widget _returnvalue))
      (UserInterface|Viewport|AddtoViewport _output_get_2 5))))