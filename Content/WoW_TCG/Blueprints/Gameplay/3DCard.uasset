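; Replicated 3D card actor for a trading card game, covering board placement, selection, attack movement, triggered abilities and graveyard exit.
; Card data from a table lookup or struct fills stats and abilities, then builds dynamic materials and text renderers.
; Authority-checked logic runs abilities and graveyard moves, with multicasts for visuals and effects.
; A tick gate interpolates movement toward a goal, then branches on movement state at arrival.
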(event Custom|Multicast_MoveToGraveyard
  ;[0.4452 0.9301 1 0.298] Multicast - Set the visual and interaction state of the card when moving to the graveyard. Move card to the graveyard.
  (Networking|CanExecuteCosmeticEvents
    (:True
      (CallFunction|EventDeselected)
      (CardData|SetTurnStateVisual false)
      (Utilities|RemoveMouseOverPreview
        (:Return
          (Collision|SetCollisionEnabled (Variables|Default|GetCard%20Base) "NoCollision")
          (Rendering|Material|SetMaterial (Variables|Default|GetCard%20Base) 0 "/Game/WoW_TCG/Materials/3DCardNothing_Mat.3DCardNothing_Mat")
          (Gameplay|PlayMovementAnimation "NewEnumerator0" "0, 0, 0" "0, 0, 0" 0 5e+01 0.001 12.0))))))

(event Custom|Open%20Gate
  (bind (_returnvalue _arrived) (CardLocationandRotation|InterpSelftoLocation))
  (bind (_returnvalue_2 _arrived_2) (CardLocationandRotation|InterpSelftoRotation))
  ;[0.4431 0.9255 1 0.298] Events - Open/ Close Gate
  ;[0.4431 0.9255 1 0.298] Gate - InterpTo Location/ Rotation
  (Utilities|FlowControl|Gate true) ; enters at Open
)

(event Custom|RemoveCardActor
  ;[1 0.5333 0.2078 0.298] Destroy Card
  (Utilities|FlowControl|Delay 0.5)
  (Actor|DestroyActor))

(event Custom|Mutlicast_SetCardVisuals
  ;[0.4431 0.9255 1 0.298] Multicast - Set Card Visuals
  (CardData|SetCardVisuals))

(event Custom|Server_ActivateAbility
  (params (AbilityIndex :type Integer))
  ;[1 0.5333 0.2078 0.298] Server - Activate Ability
  (Networking|SwitchHasAuthority
    (:Authority
      (CallFunction|MulticastAbilityVisual)
      (CallFunction|MulticastSpawnEffect "NewEnumerator0")
      (bind _succesful (CallFunction|RunCardAbility AbilityIndex))
      (if _succesful
        _))))

(event Custom|SetClientSideData
  (params (CardTableName :type Name) (CardRace :type CardSet_Variable%20Enum :default "NewEnumerator0"))
  ;[0.4431 0.9255 1 0.298] Multicast - Set Card Visuals
  (CardData|SetCardData :Card%20Table%20Name CardTableName :Card%20Set CardRace)
  (CardData|SetCardVisuals))

(event Custom|Multicast_PlaceCardOnBoard
  (params (Destination :type Vector) (Rotation :type Rotator))
  (bind _returnrotation (CallFunction|GetWorldRotationforPlayer "0, 0, 0"))
  ;[0.4431 0.9255 1 0.298] Multicast - Set home destination, rotation, and place this card on the board
  (Variables|MiscVariables|SetHomeDestination Destination)
  (if (Variables|System|GetbIsPlaced)
    _
    (else
      (Variables|System|SetbIsPlaced true)
      (Transformation|SetActorRotation _returnrotation)
      (Rendering|Material|SetMaterial (Variables|Default|GetCard%20Base) 0 (Variables|Visual|GetOuterMaterial)) ; Set Shadow Material
    ))
  (Variables|MiscVariables|SetHomeRotation (Math|Rotator|CombineRotators _returnrotation Rotation))
  (Gameplay|PlayMovementAnimation "NewEnumerator0" (Variables|MiscVariables|GetHomeDestination) (Variables|MiscVariables|GetHomeRotation) 0 5e+01 0.001 12.0))

(event Custom|ForceMoveCardDirectlyToGraveyard
  (params (Graveyard :type %20Object%20Reference))
  ;[0.4452 0.9301 1 0.298] Force Move this card directly to the graveyard. Do not pass go. Do not Collect $200.
  (Transformation|SetActorRotation "0, 0, 0")
  (Rendering|Material|SetMaterial 0 (Variables|Visual|GetOuterMaterial)) ; Set Shadow Material
  (CallFunction|PlayMovementAnimation 0 "0, 0, 0" (Transformation|GetActorRotation Graveyard) 0 5e+01 2.5 12.0))

(event Custom|Server_SetCardData
  (params (CardTableName :type Name) (CardRace :type CardSet_Variable%20Enum :default "NewEnumerator0") (CardStruct :type Card%20Struct%20Structure) (SetCardDataFromStruct :type Boolean))
  ;[1 0.5333 0.2078 0.298] Server - Set Card Data
  (Networking|SwitchHasAuthority
    (:Authority
      (CardData|SetCardData CardTableName CardRace CardStruct SetCardDataFromStruct)
      (CallFunction|MutlicastSetCardVisuals))))

(event Custom|Close%20Gate
  (bind (_returnvalue _arrived) (CardLocationandRotation|InterpSelftoLocation))
  (bind (_returnvalue_2 _arrived_2) (CardLocationandRotation|InterpSelftoRotation))
  ;[0.4431 0.9255 1 0.298] Events - Open/ Close Gate
  ;[0.4431 0.9255 1 0.298] Gate - InterpTo Location/ Rotation
  (Utilities|FlowControl|Gate true) ; enters at Close
)

(event Custom|Multicast_UpdateVisualStats
  ;[0.4431 0.9255 1 0.298] Multicast - Update Text Renderer Stats
  (Utilities|IsValid self
    (:Is%20Valid
      (Rendering|Components|TextRender|SetText (Variables|Default|GetAttack%20Text) (Utilities|Text|ToText(String) (Utilities|String|ToString(Integer) (Variables|CardData|GetAttack))))
      (Rendering|Components|TextRender|SetText (Variables|Default|GetHealth%20Text) (Utilities|Text|ToText(String) (Utilities|String|ToString(Integer) (Variables|CardData|GetHealth))))
      (Rendering|Components|TextRender|SetText (Variables|Default|GetMana%20Cost%20Text) (Utilities|Text|ToText(String) (Utilities|String|ToString(Integer) (Variables|CardData|GetMana_Cost_Placement)))))))

(event Custom|Multicast_Attacking
  (params (Attacking... :type Actor%20Object%20Reference))
  ;[0.4442 0.9233 1 0.3] Multicast - Disable collision while attacking and play movement animation
  (Networking|SwitchHasAuthority
    (:Authority
      (Networking|CanExecuteCosmeticEvents
        (:True
          _)))
    (:Remote
      _))
  (Variables|System|SetbIsAttacking true)
  (Collision|SetCollisionEnabled (Variables|Default|GetCard%20Base) "NoCollision")
  (Gameplay|PlayMovementAnimation "NewEnumerator0" "0, 0, 0" "0, 0, 0" Attacking... 5e+01 0.001 12.0))

(event Custom|Arrived%20At%20Destination
  ;[0.4431 0.9255 1 0.298] Event - Once the card has arrived at its goal destination, switch based on the current movement state
  (switch Utilities|FlowControl|Switch|Switchon (Variables|System|GetCardMovementState)
    (:NewEnumerator5)
    (:NewEnumerator1
      ;[0.4431 0.9255 1 0.298] Attacking - Once the card has reached its attacking position, move the card back to its home destination and set the card visual state
      (Variables|System|SetbIsAttacking false)
      (CallFunction|MulticastSpawnEffect "NewEnumerator0")
      (if (> (Variables|CardData|GetTurnPoints) 0)
        _
        (else
          (Variables|System|SetbCardActive false)))
      (CallFunction|PlayMovementAnimation 0 (Variables|MiscVariables|GetHomeDestination) (Variables|MiscVariables|GetHomeRotation) 0 0.0 5.0 12.0))
    (:NewEnumerator6
      ;[0.4431 0.9255 1 0.298] Card has been moved to the graveyard. Notify the graveyard of its arrival.
      (CallFunction|CloseGate)
      (Utilities|IsValid (.Placement%20Owner (Variables|System|GetPlacement%20Owner))))))

(event Custom|SpawnEffect
  (params (CardEffect :type CardEffects_Variable%20Enum :default "NewEnumerator0"))
  (bind _card_data_struct (Variables|CardData|GetCard%20Data%20Struct))
  (bind (_particle _soundcue) (CallFunction|GetCardEffectforState CardEffect _card_data_struct))
  ;[0.4431 0.9255 1 0.298] Multicast - Spawn and Play Effect
  (Networking|CanExecuteCosmeticEvents
    (:True
      (CallFunction|SpawnParticleandSoundEffect _particle "0, 0, 0" self "1.000000,1.000000,1.000000" true _soundcue 1.0))))

(event Custom|Multicast_UpdateCardVisual
  (params (IsActive :type Boolean))
  ;[0.4431 0.9255 1 0.298] Multicast - Update Turn State Visual
  (CardData|SetTurnStateVisual IsActive))

(event Custom|Multicast_AbilityVisual
  ;[1 0.5333 0.2078 0.298] Server - Activate Ability
)

(event Custom|Multicast_DamageVisual
  ;[1 0.5333 0.2078 0.298] SERVER - Recieve card damage. Set and call relevent visual events.
  (|DamageColourChange_2_2) ; Simply changes the cards colour when it takes damage for 0.1 seconds to display damage being delt.
)

(event Custom|SetCardHiddenState
  (params (bNewHidden :type Boolean))
  ;[0.4431 0.9255 1 0.298] Multicast - Set Card Hidden
  (Rendering|SetActorHiddenInGame bNewHidden)
  (Collision|SetCollisionEnabled (Variables|Default|GetCard%20Base) "NoCollision"))

(event Custom|Multicast_SpawnEffect
  (params (CardEffect :type CardEffects_Variable%20Enum :default "NewEnumerator0"))
  (bind _card_data_struct (Variables|CardData|GetCard%20Data%20Struct))
  (bind (_particle _soundcue) (CallFunction|GetCardEffectforState CardEffect _card_data_struct))
  ;[0.4431 0.9255 1 0.298] Multicast - Spawn and Play Effect
  (Networking|CanExecuteCosmeticEvents
    (:True
      (CallFunction|SpawnParticleandSoundEffect _particle "0, 0, 0" self "1.000000,1.000000,1.000000" true _soundcue 1.0))))

(event Custom|CustomEvent_3
  ;[1 0.533 0.208 0.3] Multicast - End Player Turn
  (Variables|System|SetbCardActive true))

(event Custom|CustomEvent_1
  (params (DealingCard :type %20Object%20Reference) (DamageAttack :type Integer) (DamageHealth :type Integer))
  ;[1 0.5333 0.2078 0.298] SERVER - Recieve card damage. Set and call relevent visual events.
  (Networking|SwitchHasAuthority
    (:Authority
      (Utilities|IsValid DealingCard
        (:Is%20Valid
          (Variables|Default|SetDamageDealingCard_Ref DealingCard))
        (:Is%20Not%20Valid
          (Variables|Default|SetDamageDealingCard_Ref 0))))))

(event Custom|CustomEvent_2
  ;[1 0.533 0.208 0.3] Event - Activate Turn Event
  (Networking|SwitchHasAuthority
    (:Authority
      (Variables|CardData|SetTurnPoints 1)
      (Variables|System|SetbCardActive true)
      (Utilities|ValidateAbility))))

(event EventTick
  (params (DeltaSeconds :type Float%20%28single-precision%29))
  (bind (_returnvalue _arrived) (CardLocationandRotation|InterpSelftoLocation))
  (bind (_returnvalue_2 _arrived_2) (CardLocationandRotation|InterpSelftoRotation))
  ;[0.4431 0.9255 1 0.298] Event Tick
  (Variables|System|SetDeltaTime DeltaSeconds)
  ;[0.4431 0.9255 1 0.298] Gate - InterpTo Location/ Rotation
  (Utilities|FlowControl|Gate true
    (:Exit
      (Transformation|SetActorTransform (Math|Transform|MakeTransform _returnvalue _returnvalue_2 "1,1,1"))
      (if (and _arrived _arrived_2)
        (CallFunction|ArrivedatDestination)))))

(event EventBeginPlay
  ;[0.4431 0.9255 1 0.298] Event Begin Play
  (bind _astcg_game_instance (Utilities|Casting|CastToTCG_GameInstance (Game|GetGameInstance))
    (:then
      (Variables|System|SetPlatform (.Return%20Platform (Default|GetCurrentPlatform _astcg_game_instance)))
      (Variables|System|SetbIsPlatformMobile (.Mobile? (Default|GetCurrentPlatform _astcg_game_instance))))
    (:CastFailed
      _))
  (Collision|SetCollisionEnabled (Variables|Default|GetCard%20Base) "NoCollision")
  (bind _astcg_game_state (Utilities|Casting|CastToTCG_GameState (Game|GetGameState)))
  (Variables|System|SetGameState_Ref _astcg_game_state))

(event Custom|Event_Deselected
  ;[0.4431 0.9255 1 0.298] Event - Deselected
  (if (Variables|System|GetbIsSelected)
    (Variables|System|SetbIsSelected false)
    (Transformation|SetActorScale3D "1.000000,1.000000,1.000000")
    (Rendering|Material|SetMaterial (Variables|Default|GetCard%20Base) 0 (Variables|Visual|GetOuterMaterial))))

(event Custom|Event_Selected
  (params (SelectingPlayerID :type Integer))
  ;[0.4431 0.9255 1 0.298] Event - Selected
  (if (not (Variables|System|GetbIsSelected))
    (Variables|System|SetbIsSelected true)
    (Transformation|SetActorScale3D "1.150000,1.150000,1.150000")
    (if (== SelectingPlayerID (Variables|System|GetOwningPlayerID))
      (Rendering|Material|SetMaterial (Variables|Default|GetCard%20Base) 0 "/Game/WoW_TCG/Materials/CardGreenGlow_Mat.CardGreenGlow_Mat")
      (else
        (Rendering|Material|SetMaterial (Variables|Default|GetCard%20Base) 0 "/Game/WoW_TCG/Materials/CardRedGlow_Mat.CardRedGlow_Mat")))
    (Utilities|RemoveMouseOverPreview)))

(fn ConstructionScript)

(fn SetTurnStateVisual
  (params (Is%20Active :type Boolean))
  (if Is%20Active ; Does the card have any active turn points?
    ;[0.4431 0.9255 1 0.298] Undarken Card when it has active turn points
    (Utilities|ChangeTurnStateVisual "NewEnumerator0")
    (else
      ;[0.4431 0.9255 1 0.298] Darken Card to display having no more turn points
      (Utilities|ChangeTurnStateVisual "NewEnumerator1"))))

(fn OnRepAttack)

(fn OnRepHealth)

(fn OnRepManaCostPlacement)

(fn InterpSelftoLocation
  (bind _self self)
  (bind _goaldestination (Variables|MiscVariables|GetGoalDestination))
  (bind _errortolerance (Variables|System|GetErrorTolerance))
  (bind _returnvalue (Transformation|GetActorLocation _self))
  (bind _returnvalue_2 (- _returnvalue _goaldestination))
  (bind _returnvalue_3 (Math|Vector|VectorLength _returnvalue_2))
  (bind _returnvalue_4 (Math|Float|NearlyEqual(Float) _returnvalue_3 0.0 _errortolerance))
  (return (select _returnvalue_4 _goaldestination (Math|Interpolation|VInterpTo _returnvalue _goaldestination (Variables|System|GetDeltaTime) (Variables|System|GetInterpSpeed))) _returnvalue_4))

(fn InterpSelftoRotation
  (bind _self self)
  (bind _goalrotation (Variables|MiscVariables|GetGoalRotation))
  (bind _errortolerance (Variables|System|GetErrorTolerance))
  (bind _returnvalue (/ _errortolerance 5.0))
  (bind _returnvalue_2 (Transformation|GetActorRotation _self))
  (bind _returnvalue_3 (Math|Rotator|Equal(Rotator) _returnvalue_2 _goalrotation _returnvalue))
  (return (select _returnvalue_3 _goalrotation (Math|Interpolation|RInterpTo _returnvalue_2 _goalrotation (Variables|System|GetDeltaTime) (Variables|System|GetInterpSpeed))) _returnvalue_3))

(fn PlayMovementAnimation
  (params (Card%20Movement%20State :type 3DCardMovementState_Variable%20Enum :default "NewEnumerator0") (Manual%20Goal%20Destination :type Vector) (Manual%20Goal%20Rotation :type Rotator) (OR%20Goal%20Actor :type Actor%20Object%20Reference) (Z%20Offset :type Float%20%28single-precision%29) (Error%20Tolerance :type Float%20%28single-precision%29) (Inter%20Speed :type Float%20%28single-precision%29))
  (bind _returnvalue (Transformation|GetActorLocation OR%20Goal%20Actor))
  (Variables|System|SetCardMovementState Card%20Movement%20State)
  (Utilities|IsValid OR%20Goal%20Actor ; Is the goal Actor set to be the goal Location?
    (:Is%20Valid
      (Variables|MiscVariables|SetGoalDestination (Math|Vector|MakeVector (.x _returnvalue) (.y _returnvalue) (+ (.z _returnvalue) Z%20Offset)))
      (Variables|MiscVariables|SetGoalRotation (Transformation|GetActorRotation OR%20Goal%20Actor)))
    (:Is%20Not%20Valid
      (Variables|MiscVariables|SetGoalDestination Manual%20Goal%20Destination)
      (Variables|MiscVariables|SetGoalRotation Manual%20Goal%20Rotation)))
  (Variables|System|SetErrorTolerance Error%20Tolerance)
  (Variables|System|SetInterpSpeed Inter%20Speed)
  (CallFunction|OpenGate)
  (return))

(fn OnRepOwningPlayerID)

(fn SetCardData
  (params (Card%20Table%20Name :type Name) (Card%20Set :type CardSet_Variable%20Enum :default "NewEnumerator0") (Card%20Struct :type Card%20Struct%20Structure) (Set%20Card%20Data%20From%20Struct :type Boolean))
  (if Set%20Card%20Data%20From%20Struct
    (Variables|CardData|SetCard%20Data%20Struct Card%20Struct)
    (else
      (bind _card_struct (CallFunction|GetCardData Card%20Table%20Name Card%20Set))
      (Variables|CardData|SetCard%20Data%20Struct _card_struct)))
  (Variables|CardData|SetCard%20Data%20Table%20Name Card%20Table%20Name)
  (Variables|CardData|SetCardSet Card%20Set)
  (Variables|CardData|SetName (.Name (Utilities|Struct|BreakCard_Struct (Variables|CardData|GetCard%20Data%20Struct))))
  (Variables|CardData|SetAttack (.Damage (Utilities|Struct|BreakAttack_Struct (.Attack (Utilities|Struct|BreakCard_Struct (Variables|CardData|GetCard%20Data%20Struct))))))
  (Variables|CardData|SetCanAttackPlayer (.CanAttackPlayer (Utilities|Struct|BreakAttack_Struct (.Attack (Utilities|Struct|BreakCard_Struct (Variables|CardData|GetCard%20Data%20Struct))))))
  (Variables|CardData|SetCanAttackCards (.CanAttackCards (Utilities|Struct|BreakAttack_Struct (.Attack (Utilities|Struct|BreakCard_Struct (Variables|CardData|GetCard%20Data%20Struct))))))
  (Variables|CardData|SetHealth (.Health (Utilities|Struct|BreakHealth_Struct (.Health (Utilities|Struct|BreakCard_Struct (Variables|CardData|GetCard%20Data%20Struct))))))
  (bind _output_get (Variables|CardData|SetLifeExpectancy (.LifeExpectancy (Utilities|Struct|BreakHealth_Struct (.Health (Utilities|Struct|BreakCard_Struct (Variables|CardData|GetCard%20Data%20Struct)))))))
  (Variables|System|SetbEnableLifeExpectancy (> _output_get 0))
  (Variables|CardData|SetMana_Cost_Placement (.ManaCost (Utilities|Struct|BreakPlacement_Struct (.PlacementSettings (Utilities|Struct|BreakCard_Struct (Variables|CardData|GetCard%20Data%20Struct))))))
  (Variables|CardData|SetType (.Type (Utilities|Struct|BreakCard_Struct (Variables|CardData|GetCard%20Data%20Struct))))
  (for _array_element (.Ability (Utilities|Struct|BreakCard_Struct (Variables|CardData|GetCard%20Data%20Struct)))
    (Utilities|Array|Add (Variables|Abilities|GetAbility%20Struct%20Ref) _array_element)
    (Utilities|Array|Add (Variables|Abilities|GetAbilityType%28s%29) (.Type (Utilities|Struct|BreakAbility_Struct _array_element)))
    (Utilities|Array|Add (Variables|Abilities|GetAbilityTrigger%28s%29) (.Trigger (Utilities|Struct|BreakAbility_Struct _array_element))))
  (Variables|CardData|SetDescription (Utilities|Struct|BreakDescriptions_Struct (.Description (Utilities|Struct|BreakCard_Struct (Variables|CardData|GetCard%20Data%20Struct)))))
  (return))

(fn OnRepType)

(fn SetCardVisuals
  (bind _card_data_struct (Variables|CardData|GetCard%20Data%20Struct))
  (bind (_name _class _type _rarity _special _visual _attack _health _ability _description) (Utilities|Struct|BreakCard_Struct _card_data_struct))
  (bind (_frametexture _imagetexture _backtexture _framematerial _imagematerial _backmaterial) (Utilities|Struct|BreakVisual_Struct _visual))
  (Networking|CanExecuteCosmeticEvents
    (:True
      (bind _returnvalue (Rendering|Material|CreateDynamicMaterialInstance (Variables|Default|GetCard%20Base) 1 _framematerial "None" :!class /Script/Engine.PrimitiveComponent)) ; Create dynamic Card Frame Material
      (bind _output_get (Variables|Visual|SetCardFrameMaterial _returnvalue))
      (Rendering|Material|SetMaterial (Variables|Default|GetCard%20Base) 3 _output_get) ; Set Card Frame Material
      (bind _returnvalue_2 (Rendering|Material|CreateDynamicMaterialInstance (Variables|Default|GetCard%20Base) 2 _imagematerial "None" :!class /Script/Engine.PrimitiveComponent)) ; Create dynamic Card Image Material
      (bind _output_get_2 (Variables|Visual|SetCardImageMaterial _returnvalue_2))
      (Rendering|Material|SetMaterial (Variables|Default|GetCard%20Base) 1 _output_get_2) ; Set Card Image Material
      (bind _returnvalue_3 (Rendering|Material|CreateDynamicMaterialInstance (Variables|Default|GetCard%20Base) 2 _backmaterial "None" :!class /Script/Engine.PrimitiveComponent)) ; Create dynamic Card Back Material
      (bind _output_get_3 (Variables|Visual|SetCardBackMaterial _returnvalue_3))
      (Rendering|Material|SetMaterial (Variables|Default|GetCard%20Base) 2 _output_get_3) ; Set Card Back Material
      (Rendering|Components|TextRender|SetText (Variables|Default|GetName%20Text) (Variables|CardData|GetName)) ; Set Card Name text
      (Rendering|Components|TextRender|SetText (Variables|Default|GetCard%20Type%20Text) (Utilities|Text|ToText(String) (Utilities|String|EnumtoString (Variables|CardData|GetType)))) ; Set Card Type text
      (DescriptionGenerator|GenerateDescription (Utilities|Struct|BreakDescriptions_Struct _description)) ; Create description Text Renderers for description
      (CallFunction|MulticastUpdateVisualStats)
      (Variables|Visual|SetOuterMaterial (Variables|Visual|GetShadow_Mat_Ref)))
    (:False
      _))
  (return))

(fn GenerateDescription
  (params (Description%20Text :type String))
  (Variables|Default|SetCurrentString%20Character 0)
  (for _index (range 0 (/ (Utilities|Array|Length (Utilities|String|GetCharacterArrayfromString Description%20Text)) (Variables|System|GetMax%20Description%20Character%20Line%20Length)))
    (if (== _index 0)
      (Rendering|Components|TextRender|SetText (Variables|Default|GetDescription%20Text) (Utilities|Text|ToText(String) (Utilities|String|GetSubstring Description%20Text (Variables|Default|GetCurrentString%20Character) (Variables|System|GetMax%20Description%20Character%20Line%20Length))))
      (Variables|Default|SetCurrentString%20Character (+ (Variables|Default|GetCurrentString%20Character) (Variables|System|GetMax%20Description%20Character%20Line%20Length)))
      (else
        (bind _returnvalue (AddComponent|AddTextRenderComponent false (.ReturnValue (|CalculateTextRendererTransform_2 _index Description%20Text))))
        (Rendering|Components|TextRender|SetTextRenderColor _returnvalue (Variables|/Script/Engine.TextRenderComponent|GetTextRenderColor (Variables|Default|GetDescription%20Text)))
        (Rendering|Components|TextRender|SetWorldSize _returnvalue (Variables|/Script/Engine.TextRenderComponent|GetWorldSize (Variables|Default|GetDescription%20Text)))
        (Rendering|Components|TextRender|SetText _returnvalue (Utilities|Text|ToText(String) (Utilities|String|GetSubstring (.OutputPin (|CalculateTextRendererTransform_2 _index Description%20Text)) (Variables|Default|GetCurrentString%20Character) (Variables|System|GetMax%20Description%20Character%20Line%20Length))))
        (Variables|Default|SetCurrentString%20Character (+ (Variables|Default|GetCurrentString%20Character) (Variables|System|GetMax%20Description%20Character%20Line%20Length)))))))

(fn OnRepBCardActive)

(fn MovetoGraveyard
  (bind _owningplayerid (Variables|System|GetOwningPlayerID))
  (bind _gamestate_ref (Variables|System|GetGameState_Ref))
  (bind _returngraveyard (Default|GetGraveyardReference _gamestate_ref _owningplayerid))
  (Networking|SwitchHasAuthority
    (:Authority
      (Variables|System|SetbIsPlaced false)
      (Variables|CardData|SetTurnPoints 0)
      (if (Variables|System|GetbInGraveyard)
        _
        (else
          (Variables|System|SetbInGraveyard false)))
      (Variables|System|SetCardMovementState "NewEnumerator6")
      ;[0.4431 0.9255 1 0.298] Activate 'Move to Graveyard' Ability
      (Utilities|ValidateAbility
        (:Has%20Ability
          (Utilities|RunActiveAbility "NewEnumerator5"
            (:Ran%20Ability
              _)
            (:Did%20Not%20Run%20Ability
              _)))
        (:No%20Ablity
          _))
      (Variables|Abilities|SetIsAbilityActive false)
      (if (.AddtoPlayerDeck (Utilities|Struct|BreakCard_Settings_Struct (.DeckSettings (Utilities|Struct|BreakCard_Struct (Variables|CardData|GetCard%20Data%20Struct))))) ; If the card  can be added to the deck, it can also be added to the graveyard. If not, then it will be destroyed.
        ;[0.4431 0.9255 1 0.298] Move card to graveyard (Or destroy)
        (Utilities|IsValid _returngraveyard ; If no graveyard has been selected for the placement, Destroy the card.
          (:Is%20Valid
            (Default|AddtoGraveyard _returngraveyard self "None")
            (CallFunction|MulticastMovetoGraveyard) ; Call Server event to move this card to the gravyard
          )
          (:Is%20Not%20Valid
            (CallFunction|SetCardHiddenState true :!label _label)
            (CallFunction|RemoveCardActor)))
        (else
          (goto _label))))
    (:Remote
      (return))))

(fn OnRepTurnsAlive)