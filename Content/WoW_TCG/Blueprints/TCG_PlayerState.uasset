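; Player state for the WoW TCG card game, with RepNotify handlers for hand cards, player turn, health, mana, max mana and three unnamed variables.
; All OnRep handlers are empty stubs.
; A ForceUIUpdate event calls UpdateUI, which only checks that the local player controller is a valid TCG_PlayerController.
; An ownership and empty-hand check sits unconnected, so no UI refresh logic runs here.
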(event Custom|Force%20UI%20Update
  ;[0 0.4744 1] Force UI Update
  (Utilities|UpdateUI))

(fn ConstructionScript)

(fn OnRepCardsinHandArray)

(fn OnRepPlayerTurn)

(fn OnRepNewVar5)

(fn OnRepNewVar4)

(fn OnRepNewVar3)

(fn OnRepHealth)

(fn OnRepManaMax)

(fn OnRepMana)