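; Blueprint function library for the TCG that resolves and spawns visual and audio effects for card and player states.
; Card lookups select particle and sound from the card struct's placement, attack, ability (by index) or death data; health-change slots are empty.
; Player lookups have only empty slots.
; A spawn helper plays valid particles at an actor or given location with scale, and valid sounds in 2D.
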(fn GetCardEffectforState
  (params (Effect :type CardEffects_Variable%20Enum :default "NewEnumerator0") (Card%20Struct :type Card%20Struct%20Structure) (Wild%20card%20Index :type Integer))
  (bind (_name _class _faction _type _rarity _special _visual _attack _health _ability _description _placementsettings) (Utilities|Struct|BreakCard_Struct Card%20Struct))
  (bind (_damage _manacost _canattackplayer _canattackcards _damagetype _attackparticle _attacksoundcue) (Utilities|Struct|BreakAttack_Struct _attack))
  (bind (_health_2 _lifeexpectancy _deathparticle _soundcuedeath) (Utilities|Struct|BreakHealth_Struct _health))
  (bind (_owner _manacost_2 _entryparticle _entrysoundcue) (Utilities|Struct|BreakPlacement_Struct _placementsettings))
  (bind _output (Utilities|Array|Get(acopy) _ability Wild%20card%20Index))
  (bind (_type_2 _abilityint _trigger _afterusestate _affectingplayer _particle _soundcue) (Utilities|Struct|BreakAbility_Struct _output))
  (return (Utilities|Select :Index Effect :NewEnumerator0 _entryparticle :NewEnumerator1 _attackparticle :NewEnumerator2 0 :NewEnumerator3 0 :NewEnumerator4 _particle :NewEnumerator5 _deathparticle) (Utilities|Select :Index Effect :NewEnumerator0 _entrysoundcue :NewEnumerator1 _attacksoundcue :NewEnumerator2 0 :NewEnumerator3 0 :NewEnumerator4 _soundcue :NewEnumerator5 _soundcuedeath)))

(fn GetPlayerEffectforState
  (params (Effect :type BoardPLayerEffects_Variable%20Enum :default "NewEnumerator0"))
  (return (Utilities|Select :Index Effect :NewEnumerator0 0 :NewEnumerator1 0 :NewEnumerator2 0) (Utilities|Select :Index Effect :NewEnumerator0 0 :NewEnumerator1 0 :NewEnumerator2 0)))

(fn SpawnParticleandSoundEffect
  (params (Particle%20to%20Spawn :type Particle%20System%20Object%20Reference) (Location :type Vector) (OR%20Actor%20For%20Location :type Actor%20Object%20Reference) (Scale :type Vector :default "1.000000,1.000000,1.000000") (Auto%20Destroy :type Boolean) (Sound%20Cue%20To%20Spawn :type Sound%20Cue%20Object%20Reference) (Volume :type Float%20%28single-precision%29))
  (Utilities|IsValid Particle%20to%20Spawn
    (:Is%20Valid
      (bind _returnvalue (Effects|SpawnEmitteratLocation 0 Particle%20to%20Spawn (select (Utilities|IsValid OR%20Actor%20For%20Location) (Transformation|GetActorLocation OR%20Actor%20For%20Location) Location) "0, 0, 0" "1.000000,1.000000,1.000000" Auto%20Destroy))
      (Transformation|SetWorldScale3D _returnvalue Scale))
    (:Is%20Not%20Valid
      _))
  (Utilities|IsValid Sound%20Cue%20To%20Spawn
    (:Is%20Valid
      (Audio|SpawnSound2D 0 Sound%20Cue%20To%20Spawn Volume 1.0 0.0 0))
    (:Is%20Not%20Valid
      _))
  (return))