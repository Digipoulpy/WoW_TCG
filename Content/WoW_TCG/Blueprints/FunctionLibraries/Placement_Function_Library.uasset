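; Function library for the TCG that finds and validates board placements for cards.
; Availability checks require a non-full slot supporting the card's type from card data, and filter each player's GameState placement list.
; GetClosestAvailablePlacement probes the given slot and up to five linked left and right neighbors, mixing RandomBool, FlipFlop and MultiGate to vary side order.
; The bounded search drops exhausted sides and returns the first valid slot found.
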(fn GetPlayersAvailablePlacementsforCard
  (params (PlayerID :type Integer) (CardName :type Name))
  (bind _availableplacements (LocalVariables|GetAvailablePlacements))
  (bind _astcg_game_state (Utilities|Casting|CastToTCG_GameState (Game|GetGameState)))
  (switch int PlayerID
    (:1
      (for _array_element (Variables|/Game/WoW_TCG/Blueprints/TCG_GameState.TCG_GameState_C|GetCard%20Placement%20Player1 _astcg_game_state)
        (if (CallFunction|GetIsPlacementAvailable _array_element CardName)
          (Utilities|Array|Add (LocalVariables|GetAvailablePlacements) _array_element))))
    (:2
      (for _array_element_2 (Variables|/Game/WoW_TCG/Blueprints/TCG_GameState.TCG_GameState_C|GetCard%20Placement%20Player2 _astcg_game_state)
        (if (CallFunction|GetIsPlacementAvailable _array_element_2 CardName)
          (Utilities|Array|Add (LocalVariables|GetAvailablePlacements) _array_element_2)))))
  (return _availableplacements (> (Utilities|Array|Length _availableplacements) 0)))

(fn GetDoesPlacementSupportCardType
  (params (Placement :type Card%20Placement%20Object%20Reference) (CardName :type Name))
  (bind _card_struct (CallFunction|GetCardData CardName "NewEnumerator0"))
  (return (Utilities|Array|ContainsItem (Variables|/Game/WoW_TCG/Blueprints/Gameplay/CardPlacement.CardPlacement_C|GetValidCardTypes_Array Placement) (.Type (Utilities|Struct|BreakCard_Struct _card_struct)))))

(fn GetIsPlacementAvailable
  (params (Placement :type Card%20Placement%20Object%20Reference) (CardName :type Name))
  (return (and (not (Variables|/Game/WoW_TCG/Blueprints/Gameplay/CardPlacement.CardPlacement_C|GetbIsFull Placement)) (CallFunction|GetDoesPlacementSupportCardType Placement CardName))))

(fn GetIsValidPlacement
  (params (Placement :type Card%20Placement%20Object%20Reference) (CardName :type Name) (CardSet :type CardSet_Variable%20Enum :default "NewEnumerator0"))
  (bind (_playerindex _ismulticardplacement _isfull _cardsinplacement _maxcardsinplacement _supportallcardtypes _validcardtypesarray) (Default|GetPlacementState Placement))
  (bind _returnvalue (Utilities|IsValid Placement))
  (if _returnvalue
    (bind _card_struct (CallFunction|GetCardData CardName CardSet))
    (if (>= (Utilities|Array|FindItem _validcardtypesarray (.Type (Utilities|Struct|BreakCard_Struct _card_struct))) 0)
      (return _returnvalue (and (not _isfull) (>= (Utilities|Array|FindItem _validcardtypesarray (.Type (Utilities|Struct|BreakCard_Struct _card_struct))) 0)))
      (else
        _)))
  (return false false))

(fn GetClosestAvailablePlacement
  (params (Placement :type Card%20Placement%20Object%20Reference) (CardName :type Name) (CardSet :type CardSet_Variable%20Enum :default "NewEnumerator0"))
  (bind _placement_left (Variables|/Game/WoW_TCG/Blueprints/Gameplay/CardPlacement.CardPlacement_C|GetPlacement_Left Placement))
  (bind _placement_left_2 (Variables|/Game/WoW_TCG/Blueprints/Gameplay/CardPlacement.CardPlacement_C|GetPlacement_Left Placement))
  (bind _placement_right (Variables|/Game/WoW_TCG/Blueprints/Gameplay/CardPlacement.CardPlacement_C|GetPlacement_Right Placement))
  (bind _placement_right_2 (Variables|/Game/WoW_TCG/Blueprints/Gameplay/CardPlacement.CardPlacement_C|GetPlacement_Right Placement))
  (bind _placement_right_3 (Variables|/Game/WoW_TCG/Blueprints/Gameplay/CardPlacement.CardPlacement_C|GetPlacement_Right Placement))
  (bind _placement_right_4 (Variables|/Game/WoW_TCG/Blueprints/Gameplay/CardPlacement.CardPlacement_C|GetPlacement_Right Placement))
  (bind _placement_right_5 (Variables|/Game/WoW_TCG/Blueprints/Gameplay/CardPlacement.CardPlacement_C|GetPlacement_Right Placement))
  (bind _placement_left_3 (Variables|/Game/WoW_TCG/Blueprints/Gameplay/CardPlacement.CardPlacement_C|GetPlacement_Left Placement))
  (bind _placement_left_4 (Variables|/Game/WoW_TCG/Blueprints/Gameplay/CardPlacement.CardPlacement_C|GetPlacement_Left Placement))
  (bind _placement_left_5 (Variables|/Game/WoW_TCG/Blueprints/Gameplay/CardPlacement.CardPlacement_C|GetPlacement_Left Placement))
  (bind _placement_left_6 (Variables|/Game/WoW_TCG/Blueprints/Gameplay/CardPlacement.CardPlacement_C|GetPlacement_Left _placement_left_3))
  (bind _placement_left_7 (Variables|/Game/WoW_TCG/Blueprints/Gameplay/CardPlacement.CardPlacement_C|GetPlacement_Left _placement_left_2))
  (bind _placement_right_6 (Variables|/Game/WoW_TCG/Blueprints/Gameplay/CardPlacement.CardPlacement_C|GetPlacement_Right _placement_right_3))
  (bind _placement_right_7 (Variables|/Game/WoW_TCG/Blueprints/Gameplay/CardPlacement.CardPlacement_C|GetPlacement_Right _placement_right_2))
  (bind _placement_right_8 (Variables|/Game/WoW_TCG/Blueprints/Gameplay/CardPlacement.CardPlacement_C|GetPlacement_Right _placement_right_4))
  (bind _placement_right_9 (Variables|/Game/WoW_TCG/Blueprints/Gameplay/CardPlacement.CardPlacement_C|GetPlacement_Right _placement_right_5))
  (bind _placement_left_8 (Variables|/Game/WoW_TCG/Blueprints/Gameplay/CardPlacement.CardPlacement_C|GetPlacement_Left _placement_left_4))
  (bind _placement_left_9 (Variables|/Game/WoW_TCG/Blueprints/Gameplay/CardPlacement.CardPlacement_C|GetPlacement_Left _placement_left_5))
  (bind _placement_left_10 (Variables|/Game/WoW_TCG/Blueprints/Gameplay/CardPlacement.CardPlacement_C|GetPlacement_Left _placement_left_7))
  (bind _placement_right_10 (Variables|/Game/WoW_TCG/Blueprints/Gameplay/CardPlacement.CardPlacement_C|GetPlacement_Right _placement_right_8))
  (bind _placement_right_11 (Variables|/Game/WoW_TCG/Blueprints/Gameplay/CardPlacement.CardPlacement_C|GetPlacement_Right _placement_right_7))
  (bind _placement_right_12 (Variables|/Game/WoW_TCG/Blueprints/Gameplay/CardPlacement.CardPlacement_C|GetPlacement_Right _placement_right_9))
  (bind _placement_left_11 (Variables|/Game/WoW_TCG/Blueprints/Gameplay/CardPlacement.CardPlacement_C|GetPlacement_Left _placement_left_9))
  (bind _placement_left_12 (Variables|/Game/WoW_TCG/Blueprints/Gameplay/CardPlacement.CardPlacement_C|GetPlacement_Left _placement_left_6))
  (bind _placement_left_13 (Variables|/Game/WoW_TCG/Blueprints/Gameplay/CardPlacement.CardPlacement_C|GetPlacement_Left _placement_left_10))
  (bind _placement_left_14 (Variables|/Game/WoW_TCG/Blueprints/Gameplay/CardPlacement.CardPlacement_C|GetPlacement_Left _placement_left_12))
  (bind _placement_right_13 (Variables|/Game/WoW_TCG/Blueprints/Gameplay/CardPlacement.CardPlacement_C|GetPlacement_Right _placement_right_12))
  (bind _placement_right_14 (Variables|/Game/WoW_TCG/Blueprints/Gameplay/CardPlacement.CardPlacement_C|GetPlacement_Right _placement_right_11))
  (bind _placement_right_15 (Variables|/Game/WoW_TCG/Blueprints/Gameplay/CardPlacement.CardPlacement_C|GetPlacement_Right _placement_right_14))
  (bind _placement_left_15 (Variables|/Game/WoW_TCG/Blueprints/Gameplay/CardPlacement.CardPlacement_C|GetPlacement_Left _placement_left_14))
  (LocalVariables|SetLeftValidPath true)
  (LocalVariables|SetRightValidPath true)
  (Utilities|FlowControl|ForLoopwithBreak 0 12 :!label _label ; Check is 10 layers deep
    (:LoopBody
      (if (Math|Random|RandomBool)
        (Utilities|FlowControl|FlipFlop
          (:A
            (if (LocalVariables|GetLeftValidPath) :!label _label_2
              (Utilities|FlowControl|MultiGate false false -1
                (:Out%200
                  (bind (_isvalid _validplacement) (CallFunction|GetIsValidPlacement Placement CardName CardSet))
                  (if _isvalid
                    (if _validplacement
                      (LocalVariables|SetChosenPlacement Placement)
                      (goto _label Break))
                    (else
                      (LocalVariables|SetLeftValidPath false :!label _label_3))))
                (:Out%201
                  (bind (_isvalid_2 _validplacement_2) (CallFunction|GetIsValidPlacement _placement_left CardName CardSet))
                  (if _isvalid_2
                    (if _validplacement_2
                      (LocalVariables|SetChosenPlacement _placement_left)
                      (goto _label Break))
                    (else
                      (goto _label_3))))
                (:Out%202
                  (bind (_isvalid_3 _validplacement_3) (CallFunction|GetIsValidPlacement _placement_left_8 CardName CardSet))
                  (if _isvalid_3
                    (if _validplacement_3
                      (LocalVariables|SetChosenPlacement _placement_left_8)
                      (goto _label Break))
                    (else
                      (goto _label_3))))
                (:Out%203
                  (bind (_isvalid_4 _validplacement_4) (CallFunction|GetIsValidPlacement _placement_left_11 CardName CardSet))
                  (if _isvalid_4
                    (if _validplacement_4
                      (LocalVariables|SetChosenPlacement _placement_left_11)
                      (goto _label Break))
                    (else
                      (goto _label_3))))
                (:Out%204
                  (bind (_isvalid_5 _validplacement_5) (CallFunction|GetIsValidPlacement _placement_left_13 CardName CardSet))
                  (if _isvalid_5
                    (if _validplacement_5
                      (LocalVariables|SetChosenPlacement _placement_left_13)
                      (goto _label Break))
                    (else
                      (goto _label_3))))
                (:Out%205
                  (bind (_isvalid_6 _validplacement_6) (CallFunction|GetIsValidPlacement _placement_left_15 CardName CardSet))
                  (if _isvalid_6
                    (if _validplacement_6
                      (LocalVariables|SetChosenPlacement _placement_left_15)
                      (goto _label Break))
                    (else
                      (goto _label_3)))))
              (else
                (if (LocalVariables|GetRightValidPath) :!label _label_4
                  (Utilities|FlowControl|MultiGate false false -1
                    (:Out%200
                      (bind (_isvalid_7 _validplacement_7) (CallFunction|GetIsValidPlacement Placement CardName CardSet))
                      (if _isvalid_7
                        (if _validplacement_7
                          (LocalVariables|SetChosenPlacement Placement)
                          (goto _label Break))))
                    (:Out%201
                      (bind (_isvalid_8 _validplacement_8) (CallFunction|GetIsValidPlacement _placement_right CardName CardSet))
                      (if _isvalid_8
                        (if _validplacement_8
                          (LocalVariables|SetChosenPlacement _placement_right)
                          (goto _label Break))
                        (else
                          (LocalVariables|SetRightValidPath false :!label _label_5))))
                    (:Out%202
                      (bind (_isvalid_9 _validplacement_9) (CallFunction|GetIsValidPlacement _placement_right_6 CardName CardSet))
                      (if _isvalid_9
                        (if _validplacement_9
                          (LocalVariables|SetChosenPlacement _placement_right_6)
                          (goto _label Break))
                        (else
                          (goto _label_5))))
                    (:Out%203
                      (bind (_isvalid_10 _validplacement_10) (CallFunction|GetIsValidPlacement _placement_right_10 CardName CardSet))
                      (if _isvalid_10
                        (if _validplacement_10
                          (LocalVariables|SetChosenPlacement _placement_right_10)
                          (goto _label Break))
                        (else
                          (goto _label_5))))
                    (:Out%204
                      (bind (_isvalid_11 _validplacement_11) (CallFunction|GetIsValidPlacement _placement_right_13 CardName CardSet))
                      (if _isvalid_11
                        (if _validplacement_11
                          (LocalVariables|SetChosenPlacement _placement_right_13)
                          (goto _label Break))
                        (else
                          (goto _label_5))))
                    (:Out%205
                      (bind (_isvalid_12 _validplacement_12) (CallFunction|GetIsValidPlacement _placement_right_15 CardName CardSet))
                      (if _isvalid_12
                        (if _validplacement_12
                          (LocalVariables|SetChosenPlacement _placement_right_15)
                          (goto _label Break))
                        (else
                          (goto _label_5)))))
                  (elif (LocalVariables|GetLeftValidPath)
                    (goto _label_2)
                    (else
                      (return (LocalVariables|GetChosenPlacement) (Utilities|IsValid (LocalVariables|GetChosenPlacement)))))))))
          (:B
            (goto _label_4)))
        (else
          (Utilities|FlowControl|FlipFlop
            (:A
              (goto _label_4))
            (:B
              (goto _label_2))))))
    (:Completed
      (return (LocalVariables|GetChosenPlacement) (Utilities|IsValid (LocalVariables|GetChosenPlacement))))))