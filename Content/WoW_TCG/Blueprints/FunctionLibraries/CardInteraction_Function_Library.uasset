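; Function library for the TCG that resolves card attacks on other cards and on players' health.
; Non-simple attacks validate turn points, attack, graveyard state, target health and data-driven interaction conditions, then charge a turn point and multicast the attack.
; Simple card damage skips those checks.
; Damage uses the override or the card's Attack, and successful hits are recorded to battle history on the game state, while failed validation returns the failing condition.
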(fn DealDamagetoCard
  (params (SimpleDamage :type Boolean) (TalkingCard :type 3D%20Card%20Object%20Reference) (RecievingCard :type 3D%20Card%20Object%20Reference) (DamageOverride :type Integer))
  (LocalVariables|SetInteractionTalkingCard TalkingCard)
  (LocalVariables|SetInteracitionRecievingCard RecievingCard)
  (if SimpleDamage
    ;[1 0.4639 0.1607 0.3] Attack Recieving Cards health
    (Class|CardInteractionInterface|TakesDamage(Message) (LocalVariables|GetInteracitionRecievingCard) (LocalVariables|GetInteractionTalkingCard) 0 (select (> DamageOverride 0) DamageOverride (.Attack (CallFunction|ReadInteractingCardData (LocalVariables|GetInteractionTalkingCard)))) :!label _label)
    ;[0.4374 0.9901 1 0.3] Record Battle History Result
    (bind _astcg_game_state (Utilities|Casting|CastToTCG_GameState (Game|GetGameState))
      (:then
        _)
      (:CastFailed
        (return false (LocalVariables|GetCallingCardConditionFailure) (LocalVariables|GetTalkingCardConditionFailure))))
    (else
      (if (.ReturnValue (CallFunction|ValidateCardInteraction (LocalVariables|GetInteractionTalkingCard) (LocalVariables|GetInteracitionRecievingCard)))
        (bind _success (CallFunction|ChargeInteractionPoints (LocalVariables|GetInteractionTalkingCard) 1))
        (if _success
          (Default|MulticastAttacking (LocalVariables|GetInteractionTalkingCard) (LocalVariables|GetInteracitionRecievingCard))
          (goto _label)
          (else
            _))
        (else
          (LocalVariables|SetCallingCardConditionFailure (.CallingCardConditionFailure (CallFunction|ValidateCardInteraction (LocalVariables|GetInteractionTalkingCard) (LocalVariables|GetInteracitionRecievingCard))))
          (LocalVariables|SetTalkingCardConditionFailure (.TalkingCardConditionFailure (CallFunction|ValidateCardInteraction (LocalVariables|GetInteractionTalkingCard) (LocalVariables|GetInteracitionRecievingCard))))))
      (return false (LocalVariables|GetCallingCardConditionFailure) (LocalVariables|GetTalkingCardConditionFailure))))
  (Default|RecordBattleHistory _astcg_game_state (Utilities|Struct|MakeBattleHistory_Struct (Variables|/Game/WoW_TCG/Blueprints/Gameplay/3DCard.3DCard_C|GetOwningPlayerID (LocalVariables|GetInteractionTalkingCard)) "NewEnumerator0" (Variables|/Game/WoW_TCG/Blueprints/Gameplay/3DCard.3DCard_C|GetCard%20Data%20Struct (LocalVariables|GetInteractionTalkingCard)) (Variables|/Game/WoW_TCG/Blueprints/Gameplay/3DCard.3DCard_C|GetCard%20Data%20Struct (LocalVariables|GetInteracitionRecievingCard))))
  (return true (LocalVariables|GetCallingCardConditionFailure) (LocalVariables|GetTalkingCardConditionFailure)))

(fn DealDamagetoPlayer
  (params (SimpleDamage :type Boolean) (TalkingCard :type 3D%20Card%20Object%20Reference) (BoardPlayer :type Board%20Player%20Object%20Reference) (DamageOverride :type Integer))
  (LocalVariables|SetInteractionTalkingCard TalkingCard)
  (LocalVariables|SetInteractionRecievingPlayer BoardPlayer)
  (if true
    ;[1 0.1804 0.1804 0.298] Attack Enemy Player's Health
    (Class|PlayerStateInterface|DecreasePlayerHealth(Message) (CallFunction|GetControllerPlayerState(ServerOnly) (Variables|/Game/WoW_TCG/Blueprints/Gameplay/Board_Player.Board_Player_C|GetPlayerIndex (LocalVariables|GetInteractionRecievingPlayer))) (select (> DamageOverride 0) DamageOverride (.Attack (CallFunction|ReadInteractingCardData (LocalVariables|GetInteractionTalkingCard)))) :!label _label)
    ;[0.4374 0.9901 1 0.3] Record Battle History Result
    (bind _astcg_game_state (Utilities|Casting|CastToTCG_GameState (Game|GetGameState))
      (:then
        _)
      (:CastFailed
        (return false (LocalVariables|GetConditionFailure))))
    (else
      (if (.ReturnValue (CallFunction|ValidatePlayerInteraction (LocalVariables|GetInteractionTalkingCard) (LocalVariables|GetInteractionRecievingPlayer)))
        (bind _success (CallFunction|ChargeInteractionPoints (LocalVariables|GetInteractionTalkingCard) 1))
        (if _success
          (Default|MulticastAttacking (LocalVariables|GetInteractionTalkingCard) (LocalVariables|GetInteractionRecievingPlayer))
          (goto _label)
          (else
            _))
        (else
          (LocalVariables|SetConditionFailure (.ConditionFailure (CallFunction|ValidatePlayerInteraction (LocalVariables|GetInteractionTalkingCard) (LocalVariables|GetInteractionRecievingPlayer))))))
      (return false (LocalVariables|GetConditionFailure))))
  (Default|RecordBattleHistory _astcg_game_state (Utilities|Struct|MakeBattleHistory_Struct (Variables|/Game/WoW_TCG/Blueprints/Gameplay/3DCard.3DCard_C|GetOwningPlayerID (LocalVariables|GetInteractionTalkingCard)) "NewEnumerator1" (Variables|/Game/WoW_TCG/Blueprints/Gameplay/3DCard.3DCard_C|GetCard%20Data%20Struct (LocalVariables|GetInteractionTalkingCard)) "(Name_40_4BDA39A44C24A87B09BE0698B639BB19=NSLOCTEXT(\"[6DD3DE504B5A7831FCE697AA9B1EB842]\", \"583E71454385420F44F2EC8237268C20\", \"[Name]\"),Class_16_16624419481E24FA14AAB98464005375=NewEnumerator1,Faction_43_5FE00F52476F30FE4FB28D9159DE7831=NewEnumerator0,Type_18_685B30F04AD4219A0B1183BEC566E41A=NewEnumerator2,Rarity_20_87CEC21548D01C8E42F160836479C670=NewEnumerator0,Special_21_9ED0BF3045678C66417186842A5E91BC=False,Visual_39_79279E8E4AC3FEA57BCCC3B8CCF95370=(FrameTexture_15_5ED4A8B34C62CCDA545883821E7D7039=None,ImageTexture_16_EC2BE7FE403E26B5F11838AECDB8DBB6=None,BackTexture_17_72F98ACA41BABDDA99CB6CAB89550191=None,FrameMaterial_14_EB1B8405477C94AF2DE6D7B470910A00=None,ImageMaterial_13_FC9C56364DFA12D903FA34B38C7E2D6F=None,BackMaterial_12_EDF6E09642580C8D349192988E01F59F=None),Attack_38_23DB434D45E657DF703E09956CAF7A0B=(Damage_12_E9CEEBD64A45FD439E2FA995AC7349A2=1,ManaCost_13_7A7E04D94AE0C481C0BC2B88B26004FA=0,CanAttackPlayer_14_E271380B456F66535D9C33B9B7D3FCB0=True,CanAttackCards_15_401E22EF4F8BD5CDF28E7DBD33D31FAC=True,DamageType_17_D4752CAB4A156EFFD6C0B5BD87C2C2E1=NewEnumerator0,AttackParticle_18_EB19E94C4A97785FE78D31B8493DCF5F=None,AttackSoundCue_19_D81E5E9841E75AF22E2A76A41BC5577D=None),Health_37_92A3991E49989E38D859C59AAE253938=(Health_8_20BB806341551A194C542E90CCD439ED=1,LifeExpectancy_10_0913DEA448B3CE40110B4E8C13F85088=0,DeathParticle_11_F53278494B8FE6C5F1EB87AF1F0B573C=None,SoundCueDeath_13_A192FAF943EDAE833D0646B0556964CA=None),Ability_36_7663424E4D682B12F40796B467108904=(()),Description_35_CC33C9104B347D60712727A37A01DE02=(Description_2_762A737B408AFB383678339EBEFB0515=\"\"),PlacementSettings_34_B8D6DB1D4580E6EF7C131298A64027BF=(Owner_11_597738B24192C36F42A58587F2789C64=NewEnumerator0,ManaCost_10_8C1BDDAD4EAC1AA0F275F1BEF9193240=1,EntryParticle_9_58DDC90F4030AE214A8ECE86DE32E875=None,EntrySoundCue_8_F3C7091947D7CC82CE2E27A1619D7718=None),DeckSettings_33_B9D0AD8F4F6A898E6B8B2C90B216C592=(Unlocked_5_ED0339414615E44E949A6A8EBA6A11BF=True,AddtoPlayerDeck_6_AA3673144815D8FC8859D5A7525A77DB=True,MaxNuminDeck_10_C14FD9404D182913C7134A9C4F11B95C=3,Weight_11_3515DF2848F33CF8AA40CAA0001F33F6=0,ScreenSIze_12_FA9266264518ED000F8D8FAFB5FBA944=(X=512.000000,Y=768.000000)),CardSystemData_32_71C891A0446E2EB48F416292356BDFF0=(CardPurpose_13_BF2961EB46C590B09FA7BDA34FD512ED=,CardValue_14_32F8F7BF45ED7F878D79E59851590726=0,PlayConditions_15_B6A907C74A45F12C077C24918E08A09D=,InteractionConditions_16_C293B0974BE96FF9EFC57E805002405E=))" (Variables|/Game/WoW_TCG/Blueprints/Gameplay/Board_Player.Board_Player_C|GetPlayerIndex (LocalVariables|GetInteractionRecievingPlayer))))
  (return true (LocalVariables|GetConditionFailure)))

(fn ChargeInteractionPoints
  (params (CardToCharge :type 3D%20Card%20Object%20Reference) (Cost :type Integer))
  (if (>= (Variables|/Game/WoW_TCG/Blueprints/Gameplay/3DCard.3DCard_C|GetTurnPoints CardToCharge) 1)
    (Variables|/Game/WoW_TCG/Blueprints/Gameplay/3DCard.3DCard_C|SetTurnPoints CardToCharge (- (Variables|/Game/WoW_TCG/Blueprints/Gameplay/3DCard.3DCard_C|GetTurnPoints CardToCharge) Cost))
    (return true)
    (else
      (return false))))

(fn IsSameOwningPlayer
  (params (TalkingCard :type 3D%20Card%20Object%20Reference) (RecievingCard :type 3D%20Card%20Object%20Reference))
  (return (== (Variables|/Game/WoW_TCG/Blueprints/Gameplay/3DCard.3DCard_C|GetOwningPlayerID TalkingCard) (Variables|/Game/WoW_TCG/Blueprints/Gameplay/3DCard.3DCard_C|GetOwningPlayerID RecievingCard))))

(fn ValidateCardInteractionConditions
  (params (TalkingCard :type 3D%20Card%20Object%20Reference) (RecievingCard :type 3D%20Card%20Object%20Reference) (RecievingCardConditions :type Boolean))
  (LocalVariables|SetTalkingCard_Ref TalkingCard)
  (LocalVariables|SetInteractionCondition "NewEnumerator0")
  (Utilities|IsValid RecievingCard
    (:Is%20Valid
      (LocalVariables|SetRecievingCard_Ref RecievingCard))
    (:Is%20Not%20Valid
      _))
  (LocalVariables|SetValid true)
  (bind _array_element (Utilities|Array|ForEachLoopwithBreak (select RecievingCardConditions (.InteractionConditions (Utilities|Struct|BreakCard_System_Data_Struct (.CardSystemData (Utilities|Struct|BreakCard_Struct (Variables|/Game/WoW_TCG/Blueprints/Gameplay/3DCard.3DCard_C|GetCard%20Data%20Struct (LocalVariables|GetRecievingCard_Ref)))))) (.InteractionConditions (Utilities|Struct|BreakCard_System_Data_Struct (.CardSystemData (Utilities|Struct|BreakCard_Struct (Variables|/Game/WoW_TCG/Blueprints/Gameplay/3DCard.3DCard_C|GetCard%20Data%20Struct (LocalVariables|GetTalkingCard_Ref))))))) :!label _label)
    (:LoopBody
      (LocalVariables|SetInteractionCondition _array_element)
      ;[1 0.5998 0.226 0.3] Check Condition
      (switch Utilities|FlowControl|Switch|SwitchonInteractionConditions_Variable _array_element
        (:NewEnumerator1
          (if (not (CallFunction|ConditionifPlacedonOwnedPlacement (Variables|/Game/WoW_TCG/Blueprints/Gameplay/3DCard.3DCard_C|GetOwningPlayerID (LocalVariables|GetTalkingCard_Ref)) (LocalVariables|GetRecievingCard_Ref) false))
            (LocalVariables|SetValid false :!label _label_2)
            (goto _label Break)))
        (:NewEnumerator2
          (if (not (CallFunction|ConditionifPlacedonOwnedPlacement (Variables|/Game/WoW_TCG/Blueprints/Gameplay/3DCard.3DCard_C|GetOwningPlayerID (LocalVariables|GetTalkingCard_Ref)) (LocalVariables|GetRecievingCard_Ref) true))
            (goto _label_2)))
        (:NewEnumerator3
          (if (not (CallFunction|ConditionifRecievingCardType (LocalVariables|GetRecievingCard_Ref) "NewEnumerator2"))
            (goto _label_2)))
        (:NewEnumerator4
          (if (not (CallFunction|ConditionIsNotOwningPlayer (Variables|/Game/WoW_TCG/Blueprints/Gameplay/3DCard.3DCard_C|GetOwningPlayerID (LocalVariables|GetTalkingCard_Ref)) (LocalVariables|GetRecievingCard_Ref)))
            (goto _label_2)))))
    (:Completed
      (if (LocalVariables|GetValid)
        (LocalVariables|SetInteractionCondition "NewEnumerator0"))
      (return (LocalVariables|GetValid) (LocalVariables|GetInteractionCondition)))))

(fn ValidatePlayerInteraction
  (params (TalkingCard :type 3D%20Card%20Object%20Reference) (RecievingBoard%20Player :type Board%20Player%20Object%20Reference))
  (bind (_returnvalid _conditionfailure) (CallFunction|ValidateCardInteractionConditions TalkingCard 0 false))
  (return (Math|Boolean|ANDBoolean (Math|Boolean|ANDBoolean (> (Variables|/Game/WoW_TCG/Blueprints/Gameplay/3DCard.3DCard_C|GetTurnPoints TalkingCard) 0) (> (Variables|/Game/WoW_TCG/Blueprints/Gameplay/3DCard.3DCard_C|GetAttack TalkingCard) 0) (not (Variables|/Game/WoW_TCG/Blueprints/Gameplay/3DCard.3DCard_C|GetbInGraveyard TalkingCard)) (.CanAttackPlayer (Utilities|Struct|BreakAttack_Struct (.Attack (Utilities|Struct|BreakCard_Struct (Variables|/Game/WoW_TCG/Blueprints/Gameplay/3DCard.3DCard_C|GetCard%20Data%20Struct TalkingCard)))))) (> (.Health (CallFunction|GetControllersStateProfile(ServerOnly) (Variables|/Game/WoW_TCG/Blueprints/Gameplay/Board_Player.Board_Player_C|GetPlayerIndex RecievingBoard%20Player))) 0) _returnvalid) _conditionfailure))

(fn ValidateCardInteraction
  (params (TalkingCard :type 3D%20Card%20Object%20Reference) (RecievingCard :type 3D%20Card%20Object%20Reference))
  (bind (_returnvalid _conditionfailure) (CallFunction|ValidateCardInteractionConditions TalkingCard RecievingCard true))
  (bind (_returnvalid_2 _conditionfailure_2) (CallFunction|ValidateCardInteractionConditions TalkingCard RecievingCard false))
  (return (Math|Boolean|ANDBoolean (Math|Boolean|ANDBoolean (> (Variables|/Game/WoW_TCG/Blueprints/Gameplay/3DCard.3DCard_C|GetTurnPoints TalkingCard) 0) (> (Variables|/Game/WoW_TCG/Blueprints/Gameplay/3DCard.3DCard_C|GetAttack TalkingCard) 0) (not (Variables|/Game/WoW_TCG/Blueprints/Gameplay/3DCard.3DCard_C|GetbInGraveyard TalkingCard)) (.CanAttackCards (Utilities|Struct|BreakAttack_Struct (.Attack (Utilities|Struct|BreakCard_Struct (Variables|/Game/WoW_TCG/Blueprints/Gameplay/3DCard.3DCard_C|GetCard%20Data%20Struct TalkingCard)))))) (and (> (Variables|/Game/WoW_TCG/Blueprints/Gameplay/3DCard.3DCard_C|GetHealth RecievingCard) 0) (not (Variables|/Game/WoW_TCG/Blueprints/Gameplay/3DCard.3DCard_C|GetbInGraveyard RecievingCard))) (and _returnvalid_2 _returnvalid)) _conditionfailure_2 _conditionfailure))