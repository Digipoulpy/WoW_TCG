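; Blueprint function library for the WoW TCG game that writes card and ability events to a player's message log.
; AddMessageToLog checks that the calling player's game UI and its MessageManager are valid, then forwards the message and color to LogMessage.
; Helper functions use FormatText to build message strings for card cloning, card pickup and attack increases from a card name or ability value.
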(fn AddMessagetoLog
  (params (CallingPlayer :type TCG%20Player%20Controller%20Object%20Reference) (Message :type String) (Specified%20Color :type Linear%20Color%20Structure))
  (bind _player_game_ui_ref (Variables|/Game/WoW_TCG/Blueprints/TCG_PlayerController.TCG_PlayerController_C|GetPlayer%20Game%20UI%20Ref CallingPlayer))
  (bind _message_manager (Variables|/Game/WoW_TCG/Blueprints/Widgets/Player_Game_UI.Player_Game_UI_C|GetMessage_Manager _player_game_ui_ref))
  (Utilities|IsValid _player_game_ui_ref
    (:Is%20Valid
      (Utilities|IsValid _message_manager
        (:Is%20Valid
          (Default|LogMessage _message_manager CallingPlayer Message Specified%20Color))
        (:Is%20Not%20Valid
          _)))
    (:Is%20Not%20Valid
      _))
  (return))

(fn CloneCardLogMessage
  (params (CardName :type Text) (AbilityInt :type Integer))
  (return (Utilities|String|ToString(Text) (Utilities|Text|FormatText "{cardname} cloned up to + {AbilityInt} times!" CardName (Utilities|Text|ToText(Integer) AbilityInt)))))

(fn PickupCard(s)LogMessage
  (params (AbilityInt :type Integer))
  (return (Utilities|String|ToString(Text) (Utilities|Text|FormatText "Player picked up + {AbilityInt} cards" (Utilities|Text|ToText(Integer) AbilityInt)))))

(fn IncreaseAttackLogMessage
  (params (CardName :type Text) (AbilityInt :type Integer))
  (return (Utilities|String|ToString(Text) (Utilities|Text|FormatText "{cardname} gained + {AbilityInt} Attack" CardName (Utilities|Text|ToText(Integer) AbilityInt)))))