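; Function library of evaluation rules for the WoW TCG card game, turning board states and attack outcomes into point scores.
; Rules score active cards, hand size, health, card attacks and player damage, returning a running total plus the rule's own score.
; Attack rules flag removal from play, and card attacks penalise overkill.
; Two functions offset scores by the receiving card's abilities, with the owned-card variant also flagging beneficial interactions.
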(fn RuleCalculateActiveCardPoints
  (params (Add :type Integer) (PtsPerActiveCard :type Integer) (CardsActive :type Array%20of%203D%20Card%20Object%20References) (IncludePlayValue :type Boolean))
  (bind _returnvalue (Utilities|Array|Length CardsActive))
  (bind _returnvalue_2 (* PtsPerActiveCard _returnvalue))
  (bind _returnvalue_3 (+ Add _returnvalue_2))
  (if (not IncludePlayValue)
    (return _returnvalue_3 _returnvalue_2)
    (else
      (for _array_element CardsActive
        (LocalVariables|SetTEMP_CardValueTotal (+ (LocalVariables|GetTEMP_CardValueTotal) (.CardValue (Utilities|Struct|BreakCard_System_Data_Struct (.CardSystemData (Utilities|Struct|BreakCard_Struct (Variables|/Game/WoW_TCG/Blueprints/Gameplay/3DCard.3DCard_C|GetCard%20Data%20Struct _array_element))))))))
      (return (+ _returnvalue_3 (LocalVariables|GetTEMP_CardValueTotal)) (+ _returnvalue_3 (LocalVariables|GetTEMP_CardValueTotal))))))

(fn RuleCalculateCardsinHandPoints
  (params (Add :type Integer) (PtsPerCardnHand :type Integer) (CardsInHand :type Integer))
  (bind _returnvalue (* PtsPerCardnHand CardsInHand))
  (return (+ Add _returnvalue) _returnvalue))

(fn RuleCalculateHealthPoints
  (params (Add :type Integer) (PtsPerHealthPoint :type Integer) (PlayerHealth :type Integer))
  (bind _returnvalue (* PtsPerHealthPoint PlayerHealth))
  (return (+ Add _returnvalue) _returnvalue))

(fn RuleCalculateAttackPoints
  (params (Add :type Integer) (PtsForDamage :type Integer) (PtsForRemovingCardFromPlay :type Integer) (Attack :type Integer) (Health :type Integer) (CardValue :type Integer) (IncludeCardValue :type Boolean))
  (bind _returnvalue (- Health Attack))
  (bind _returnvalue_2 (select IncludeCardValue CardValue 0))
  (bind _returnvalue_3 (< _returnvalue 0))
  (bind _returnvalue_4 (Math|Integer|Absolute(Integer) _returnvalue))
  (bind _returnvalue_5 (<= _returnvalue 0))
  (bind _returnvalue_6 (select _returnvalue_5 PtsForRemovingCardFromPlay PtsForDamage))
  (bind _returnvalue_7 (select _returnvalue_3 _returnvalue_4 0))
  (bind _returnvalue_8 (+ _returnvalue_6 _returnvalue_2))
  (bind _returnvalue_9 (- _returnvalue_8 _returnvalue_7))
  (return (+ Add _returnvalue_9) _returnvalue_9 _returnvalue_5))

(fn RuleCalculateDamagetoPlayerPoints
  (params (Add :type Integer) (PtsForPlayerDamage :type Integer) (PtsForRemovingPlayer :type Integer) (CardAttack :type Integer) (PlayerHealth :type Integer))
  (bind _returnvalue (- PlayerHealth CardAttack))
  (bind _returnvalue_2 (* PtsForPlayerDamage CardAttack))
  (bind _returnvalue_3 (<= _returnvalue 0))
  (bind _returnvalue_4 (select _returnvalue_3 PtsForRemovingPlayer _returnvalue_2))
  (return (+ Add _returnvalue_4) _returnvalue_4 _returnvalue_3))

(fn RuleCalculateAdditionalAbilityPointOffset
  (params (TalkingCard :type 3D%20Card%20Object%20Reference) (RecievingCard :type 3D%20Card%20Object%20Reference))
  (LocalVariables|SetReturnPoints 0)
  (for _array_element (.Ability (Utilities|Struct|BreakCard_Struct (Variables|/Game/WoW_TCG/Blueprints/Gameplay/3DCard.3DCard_C|GetCard%20Data%20Struct RecievingCard)))
    (switch Utilities|FlowControl|Switch|SwitchonAbilityType_Variable (.Type (Utilities|Struct|BreakAbility_Struct _array_element))
      (:NewEnumerator2
        (switch Utilities|FlowControl|Switch|SwitchonAbilityTrigger_Variable (.Trigger (Utilities|Struct|BreakAbility_Struct _array_element))
          (:NewEnumerator4
            ;[1 0.5486 0.166 0.3] Increase Attack - Takes Damage
            (LocalVariables|SetReturnPoints (- (LocalVariables|GetReturnPoints) (* (Class|KismetSystemLibrary|MakeLiteralInteger 1) (.AbilityInt (Utilities|Struct|BreakAbility_Struct _array_element))))))))
      (:NewEnumerator5
        ;[1 0.5486 0.166 0.3] Retaliation Damage - All Triggers
        (LocalVariables|SetReturnPoints (- (LocalVariables|GetReturnPoints) (* (Class|KismetSystemLibrary|MakeLiteralInteger 1) (.AbilityInt (Utilities|Struct|BreakAbility_Struct _array_element))))))
      (:NewEnumerator6
        (switch Utilities|FlowControl|Switch|SwitchonAbilityTrigger_Variable (.Trigger (Utilities|Struct|BreakAbility_Struct _array_element))
          (:NewEnumerator2
            _)
          (:NewEnumerator6
            _))
        ;[1 0.5486 0.166 0.3] Damage All Cards on the board (Start of Turn, Death By Life Expectancy)
        (LocalVariables|SetReturnPoints (* (+ (LocalVariables|GetReturnPoints) 5) (.AbilityInt (Utilities|Struct|BreakAbility_Struct _array_element)))))))
  (return (LocalVariables|GetReturnPoints)))

(fn RuleCalculateOwnedCardAbilityPointOffset
  (params (TalkingCard :type 3D%20Card%20Object%20Reference) (RecievingCard :type 3D%20Card%20Object%20Reference))
  (bind _card_data_struct (Variables|/Game/WoW_TCG/Blueprints/Gameplay/3DCard.3DCard_C|GetCard%20Data%20Struct RecievingCard))
  (bind (_name _class _faction _type _rarity _special _visual _attack _health _ability) (Utilities|Struct|BreakCard_Struct _card_data_struct))
  (LocalVariables|SetReturnPoints 0)
  (for _array_element _ability
    (switch Utilities|FlowControl|Switch|SwitchonAbilityType_Variable (.Type (Utilities|Struct|BreakAbility_Struct _array_element))
      (:NewEnumerator2
        (switch Utilities|FlowControl|Switch|SwitchonAbilityTrigger_Variable (.Trigger (Utilities|Struct|BreakAbility_Struct _array_element))
          (:NewEnumerator4
            ;[1 0.5486 0.166 0.3] Increase Attack - Takes Damage
            (LocalVariables|SetReturnPoints (+ (LocalVariables|GetReturnPoints) (select (<= (- (.Health (Utilities|Struct|BreakHealth_Struct _health)) (.Damage (Utilities|Struct|BreakAttack_Struct (.Attack (Utilities|Struct|BreakCard_Struct (Variables|/Game/WoW_TCG/Blueprints/Gameplay/3DCard.3DCard_C|GetCard%20Data%20Struct TalkingCard)))))) 0) -99 5))))))
      (:NewEnumerator5
        ;[1 0.5486 0.166 0.3] Retaliation Damage - All Triggers
        (LocalVariables|SetReturnPoints (- (LocalVariables|GetReturnPoints) (* (Class|KismetSystemLibrary|MakeLiteralInteger 10) (.AbilityInt (Utilities|Struct|BreakAbility_Struct _array_element))))))
      (:NewEnumerator6
        (switch Utilities|FlowControl|Switch|SwitchonAbilityTrigger_Variable (.Trigger (Utilities|Struct|BreakAbility_Struct _array_element))
          (:NewEnumerator2
            _)
          (:NewEnumerator6
            _))
        ;[1 0.5486 0.166 0.3] Damage All Cards on the board (Start of Turn, Death By Life Expectancy)
        (LocalVariables|SetReturnPoints (* (+ (LocalVariables|GetReturnPoints) 5) (.AbilityInt (Utilities|Struct|BreakAbility_Struct _array_element)))))))
  (return (LocalVariables|GetReturnPoints) (>= (LocalVariables|GetReturnPoints) 0)))