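; Function library for the card game that lets gameplay code treat human and AI players alike through numeric IDs.
; Server-only helpers resolve IDs via the GameMode controller array, casting to player controller and state or to AI controller and pawn to fetch stats, decks and hands.
; Opponent helpers assume two seats.
; A replicated getter reads the GameState player array, falling back to a "NO OPPONENT" profile.
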(fn GetControllerID(ServerOnly)
  (params (Controller :type Controller%20Object%20Reference))
  (bind _astcg_player_controller (Utilities|Casting|CastToTCG_PlayerController Controller)
    (:then
      (bind _astcg_player_state (Utilities|Casting|CastToTCG_PlayerState (Variables|/Script/Engine.Controller|GetPlayerState _astcg_player_controller))
        (:then
          (return (Variables|/Game/WoW_TCG/Blueprints/TCG_PlayerState.TCG_PlayerState_C|GetTCG%20Player%20ID _astcg_player_state)))
        (:CastFailed
          _)))
    (:CastFailed
      (bind _astcg_ai_controller (Utilities|Casting|CastToTCG_AI_Controller Controller)
        (:then
          (bind _astcg_ai_pawn (Utilities|Casting|CastToTCG_AI_Pawn (Pawn|GetControlledPawn _astcg_ai_controller))
            (:then
              (return (Variables|/Game/WoW_TCG/TCG_AI/AI_Blueprint/TCG_AI_Pawn.TCG_AI_Pawn_C|GetPlayer%20ID _astcg_ai_pawn)))
            (:CastFailed
              _)))
        (:CastFailed
          _))))
  (Development|PrintString 0 "Failed to get Controller")
  (return -1))

(fn GetPlayerControllerReference(ServerOnly)
  (params (Controller :type Controller%20Object%20Reference))
  (bind _astcg_player_controller (Utilities|Casting|CastToTCG_PlayerController Controller)
    (:then
      (bind _astcg_player_state (Utilities|Casting|CastToTCG_PlayerState (Variables|/Script/Engine.Controller|GetPlayerState _astcg_player_controller))
        (:then
          (return _astcg_player_controller _astcg_player_state true))
        (:CastFailed
          _)))
    (:CastFailed
      _))
  (return 0 0 false))

(fn GetAiControllerReference(ServerOnly)
  (params (Controller :type Controller%20Object%20Reference))
  (bind _astcg_ai_controller (Utilities|Casting|CastToTCG_AI_Controller Controller)
    (:then
      (bind _astcg_ai_pawn (Utilities|Casting|CastToTCG_AI_Pawn (Pawn|GetControlledPawn _astcg_ai_controller))
        (:then
          (return _astcg_ai_controller _astcg_ai_pawn true))
        (:CastFailed
          _)))
    (:CastFailed
      _))
  (return 0 0 false))

(fn GetControllerReferencefromID(ServerOnly)
  (params (Controller%20ID :type Integer))
  (bind _astcg_game_mode (Utilities|Casting|CastToTCG_GameMode (Game|GetGameMode))
    (:then
      (return (Utilities|Array|Get(acopy) (Variables|/Game/WoW_TCG/Blueprints/TCG_GameMode.TCG_GameMode_C|GetGame%20Controllers%20Array _astcg_game_mode) (- Controller%20ID 1))))
    (:CastFailed
      (return 0))))

(fn GetControllersStateProfile(ServerOnly)
  (params (Controller%20ID :type Integer))
  (bind _controller (CallFunction|GetControllerReferencefromID(ServerOnly) Controller%20ID))
  (bind (_tcg_player_controller _tcg_player_state _valid) (CallFunction|GetPlayerControllerReference(ServerOnly) _controller))
  (bind (_tcg_ai_controller _tcg_ai_pawn _valid_2) (CallFunction|GetAiControllerReference(ServerOnly) _controller))
  (if _valid
    (return (Variables|/Game/WoW_TCG/Blueprints/TCG_PlayerState.TCG_PlayerState_C|GetHealth _tcg_player_state) (Variables|/Game/WoW_TCG/Blueprints/TCG_PlayerState.TCG_PlayerState_C|GetCards%20In%20Hand _tcg_player_state) (Variables|/Game/WoW_TCG/Blueprints/TCG_PlayerState.TCG_PlayerState_C|GetCards%20In%20Deck _tcg_player_state) (Variables|/Game/WoW_TCG/Blueprints/TCG_PlayerState.TCG_PlayerState_C|GetActive%20Cards _tcg_player_state) (Variables|/Game/WoW_TCG/Blueprints/TCG_PlayerState.TCG_PlayerState_C|GetMana _tcg_player_state) (Variables|/Game/WoW_TCG/Blueprints/TCG_PlayerState.TCG_PlayerState_C|GetMana%20Max _tcg_player_state) (Variables|/Game/WoW_TCG/Blueprints/TCG_PlayerState.TCG_PlayerState_C|GetPlayer%20Turn _tcg_player_state) (Variables|/Game/WoW_TCG/Blueprints/TCG_PlayerController.TCG_PlayerController_C|GetPlayer%20Deck _tcg_player_controller) (Variables|/Game/WoW_TCG/Blueprints/TCG_PlayerController.TCG_PlayerController_C|GetCards%20In%20Hand _tcg_player_controller) _tcg_player_state)
    (elif _valid_2
      (return (Variables|/Game/WoW_TCG/TCG_AI/AI_Blueprint/TCG_AI_Pawn.TCG_AI_Pawn_C|GetHealth _tcg_ai_pawn) (Variables|/Game/WoW_TCG/TCG_AI/AI_Blueprint/TCG_AI_Pawn.TCG_AI_Pawn_C|GetCards%20In%20Hand _tcg_ai_pawn) (Variables|/Game/WoW_TCG/TCG_AI/AI_Blueprint/TCG_AI_Pawn.TCG_AI_Pawn_C|GetCards%20in%20Deck _tcg_ai_pawn) (Variables|/Game/WoW_TCG/TCG_AI/AI_Blueprint/TCG_AI_Pawn.TCG_AI_Pawn_C|GetActiveCards _tcg_ai_pawn) (Variables|/Game/WoW_TCG/TCG_AI/AI_Blueprint/TCG_AI_Pawn.TCG_AI_Pawn_C|GetMana _tcg_ai_pawn) (Variables|/Game/WoW_TCG/TCG_AI/AI_Blueprint/TCG_AI_Pawn.TCG_AI_Pawn_C|GetManaMax _tcg_ai_pawn) (Variables|/Game/WoW_TCG/TCG_AI/AI_Blueprint/TCG_AI_Pawn.TCG_AI_Pawn_C|GetPlayer%20Turn _tcg_ai_pawn) (Variables|/Game/WoW_TCG/TCG_AI/AI_Blueprint/TCG_AI_Controller.TCG_AI_Controller_C|GetAI%20Deck _tcg_ai_controller) (Variables|/Game/WoW_TCG/TCG_AI/AI_Blueprint/TCG_AI_Controller.TCG_AI_Controller_C|GetAI%20Cards%20In%20Hand _tcg_ai_controller) _tcg_ai_pawn))))

(fn GetControllerIDforBothPlayers(ServerOnly)
  (params (Controller :type Controller%20Object%20Reference))
  (if (> (Utilities|Array|Length (Variables|/Game/WoW_TCG/Blueprints/TCG_GameMode.TCG_GameMode_C|GetGame%20Controllers%20Array (.AsTCG%20Game%20Mode (Utilities|Casting|CastToTCG_GameMode (Game|GetGameMode))))) 1)
    (if (== (CallFunction|GetControllerID(ServerOnly) Controller) 1)
      (return 1 2)
      (else
        (return 2 1)))
    (else
      (return 1 1))))

(fn GetControllerPlayerState(ServerOnly)
  (params (Controller :type Integer))
  (bind _controller (CallFunction|GetControllerReferencefromID(ServerOnly)))
  (bind (_tcg_player_controller _tcg_player_state _valid) (CallFunction|GetPlayerControllerReference(ServerOnly) _controller))
  (bind (_tcg_ai_controller _tcg_ai_pawn _valid_2) (CallFunction|GetAiControllerReference(ServerOnly) _controller))
  (if _valid
    (return _tcg_player_state)
    (elif _valid_2
      (return _tcg_ai_pawn))))

(fn GetReplicatedPlayerState
  (params (Player%20ID :type Integer))
  (bind _astcg_game_state (Utilities|Casting|CastToTCG_GameState (Game|GetGameState))
    (:then
      (if (>= (Utilities|Array|Length (Variables|/Game/WoW_TCG/Blueprints/TCG_GameState.TCG_GameState_C|GetPlayer%20State%20Array _astcg_game_state)) Player%20ID)
        (bind _astcg_player_state (Utilities|Casting|CastToTCG_PlayerState (Utilities|Array|Get(acopy) (Variables|/Game/WoW_TCG/Blueprints/TCG_GameState.TCG_GameState_C|GetPlayer%20State%20Array _astcg_game_state) (- Player%20ID 1)))
          (:then
            (return (Variables|/Game/WoW_TCG/Blueprints/TCG_PlayerState.TCG_PlayerState_C|GetPlayer%20Name _astcg_player_state) (Variables|/Game/WoW_TCG/Blueprints/TCG_PlayerState.TCG_PlayerState_C|GetHealth _astcg_player_state) (Variables|/Game/WoW_TCG/Blueprints/TCG_PlayerState.TCG_PlayerState_C|GetMana _astcg_player_state) (Variables|/Game/WoW_TCG/Blueprints/TCG_PlayerState.TCG_PlayerState_C|GetMana%20Max _astcg_player_state) (Variables|/Game/WoW_TCG/Blueprints/TCG_PlayerState.TCG_PlayerState_C|GetCards%20In%20Deck _astcg_player_state) (Variables|/Game/WoW_TCG/Blueprints/TCG_PlayerState.TCG_PlayerState_C|GetPlayer%20Turn _astcg_player_state) (Variables|/Game/WoW_TCG/Blueprints/TCG_PlayerState.TCG_PlayerState_C|GetCards%20In%20Hand _astcg_player_state)))
          (:CastFailed
            (bind _astcg_ai_pawn (Utilities|Casting|CastToTCG_AI_Pawn (Utilities|Array|Get(acopy) (Variables|/Game/WoW_TCG/Blueprints/TCG_GameState.TCG_GameState_C|GetPlayer%20State%20Array _astcg_game_state) (- Player%20ID 1)))
              (:then
                (return (Variables|/Game/WoW_TCG/TCG_AI/AI_Blueprint/TCG_AI_Pawn.TCG_AI_Pawn_C|GetAI_Name _astcg_ai_pawn) (Variables|/Game/WoW_TCG/TCG_AI/AI_Blueprint/TCG_AI_Pawn.TCG_AI_Pawn_C|GetHealth _astcg_ai_pawn) (Variables|/Game/WoW_TCG/TCG_AI/AI_Blueprint/TCG_AI_Pawn.TCG_AI_Pawn_C|GetMana _astcg_ai_pawn) (Variables|/Game/WoW_TCG/TCG_AI/AI_Blueprint/TCG_AI_Pawn.TCG_AI_Pawn_C|GetManaMax _astcg_ai_pawn) (Variables|/Game/WoW_TCG/TCG_AI/AI_Blueprint/TCG_AI_Pawn.TCG_AI_Pawn_C|GetCards%20in%20Deck _astcg_ai_pawn) (Variables|/Game/WoW_TCG/TCG_AI/AI_Blueprint/TCG_AI_Pawn.TCG_AI_Pawn_C|GetPlayer%20Turn _astcg_ai_pawn) (Variables|/Game/WoW_TCG/TCG_AI/AI_Blueprint/TCG_AI_Pawn.TCG_AI_Pawn_C|GetCards%20In%20Hand _astcg_ai_pawn)))
              (:CastFailed
                _))))))
    (:CastFailed
      _))
  (return "NO OPPONENT" 0 0 0 0 0 0))

(fn GetOpponentID(ServerOnly)
  (params (Playerd%20ID :type Integer))
  (if (> (Utilities|Array|Length (Variables|/Game/WoW_TCG/Blueprints/TCG_GameMode.TCG_GameMode_C|GetGame%20Controllers%20Array (.AsTCG%20Game%20Mode (Utilities|Casting|CastToTCG_GameMode (Game|GetGameMode))))) 1)
    (if (== Playerd%20ID 1)
      (return 2)
      (else
        (return 1)))
    (else
      (return 1))))