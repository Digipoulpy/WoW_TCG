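; Blueprint function library of boolean condition checks for cards in the TCG, covering board card types, player health, AI play-loop stage, placement or card ownership, and graveyard size.
; Checks read GameState, GameMode and player profiles, mostly through server-only lookups.
; AI-only checks read the board, graveyard or AI Blackboard, and return true for non-AI controllers.
; The low-playable-hand check has a hard-coded false branch, so it always returns true.
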(fn ConditionifCardTypeinPlay
  (params (Controller :type Controller%20Object%20Reference) (MinCreaturesOnBoard :type Integer) (bOpponent :type Boolean) (CardType :type CardType_Variable%20Enum :default "NewEnumerator0") (AI_Only :type Boolean))
  (if AI_Only
    (if (.Valid (CallFunction|GetAiControllerReference(ServerOnly) Controller))
      _
      (else
        (return true))))
  (bind (_selfplayer _oppenent) (CallFunction|GetPlayerStateReference Controller))
  (LocalVariables|SetCardArray (.PlayerCards (Default|GetBoardState (.AsTCG%20Game%20State (Utilities|Casting|CastToTCG_GameState (Game|GetGameState))) (select bOpponent _oppenent _selfplayer))))
  (for _array_element (LocalVariables|GetCardArray)
    (if (Utilities|Enum|Equal(Enum) (.Type (Utilities|Struct|BreakCard_Struct (Variables|/Game/WoW_TCG/Blueprints/Gameplay/3DCard.3DCard_C|GetCard%20Data%20Struct _array_element))) CardType)
      (Math|Integer|IncrementInt (LocalVariables|GetCreaturesOnBoard))))
  (return (>= (LocalVariables|GetCreaturesOnBoard) MinCreaturesOnBoard)))

(fn ConditionifPlayerLowHealth
  (params (Player%20ID :type Integer))
  (return (<= (/ (Math|Conversions|ToFloat(Integer) (.Health (CallFunction|GetControllersStateProfile(ServerOnly) Player%20ID))) (Math|Conversions|ToFloat(Integer) (Variables|/Game/WoW_TCG/Blueprints/TCG_GameMode.TCG_GameMode_C|GetPlayerStartingHealth (.AsTCG%20Game%20Mode (Utilities|Casting|CastToTCG_GameMode (Game|GetGameMode)))))) 0.35)))

(fn ConditionifPlayerHighHealth
  (params (Player%20ID :type Integer))
  (return (>= (/ (Math|Conversions|ToFloat(Integer) (.Health (CallFunction|GetControllersStateProfile(ServerOnly) Player%20ID))) (Math|Conversions|ToFloat(Integer) (Variables|/Game/WoW_TCG/Blueprints/TCG_GameMode.TCG_GameMode_C|GetPlayerStartingHealth (.AsTCG%20Game%20Mode (Utilities|Casting|CastToTCG_GameMode (Game|GetGameMode)))))) 0.7)))

(fn ConditionifStartOfPlay(AIOnly)
  (params (Player%20ID :type Integer))
  (bind _controller (CallFunction|GetControllerReferencefromID(ServerOnly) Player%20ID))
  (bind (_tcg_ai_controller _tcg_ai_pawn _valid) (CallFunction|GetAiControllerReference(ServerOnly) _controller))
  (if _valid
    (return (<= (Class|BlackboardComponent|GetValueasInt (AI|GetBlackboard _tcg_ai_controller) (Utilities|Name|MakeLiteralName "Loop")) 2))
    (else
      (return true))))

(fn ConditionifEndOfPlay(AIOnly)
  (params (Player%20ID :type Integer))
  (bind _controller (CallFunction|GetControllerReferencefromID(ServerOnly) Player%20ID))
  (bind (_tcg_ai_controller _tcg_ai_pawn _valid) (CallFunction|GetAiControllerReference(ServerOnly) _controller))
  (if _valid
    (return (ScalableFloat|GetValueasBool (AI|GetBlackboard _tcg_ai_controller) (Utilities|Name|MakeLiteralName "bFinalLoop")))
    (else
      (return true))))

(fn ConditionifPlacedonOwnedPlacement
  (params (PlayerID :type Integer) (Recieving%20Card :type 3D%20Card%20Object%20Reference) (Oppenent :type Boolean))
  (bind _placement_owner (Variables|/Game/WoW_TCG/Blueprints/Gameplay/3DCard.3DCard_C|GetPlacement%20Owner Recieving%20Card))
  (bind _playerindex (Variables|/Game/WoW_TCG/Blueprints/Gameplay/CardPlacement.CardPlacement_C|GetPlayerIndex _placement_owner))
  (Utilities|IsValid Recieving%20Card
    (:Is%20Valid
      (return (or (select Oppenent (!= PlayerID _playerindex) (== PlayerID _playerindex)) (== _playerindex 0))))
    (:Is%20Not%20Valid
      (return true))))

(fn ConditionifRecievingCardType
  (params (RecievingCard :type 3D%20Card%20Object%20Reference) (RecievingCardType :type CardType_Variable%20Enum :default "NewEnumerator0"))
  (return (Utilities|Enum|Equal(Enum) (Variables|/Game/WoW_TCG/Blueprints/Gameplay/3DCard.3DCard_C|GetType RecievingCard) RecievingCardType)))

(fn ConditionIsNotOwningPlayer
  (params (PlayerID :type Integer) (RecievingCard :type 3D%20Card%20Object%20Reference))
  (Utilities|IsValid RecievingCard
    (:Is%20Valid
      (return (!= PlayerID (Variables|/Game/WoW_TCG/Blueprints/Gameplay/3DCard.3DCard_C|GetOwningPlayerID RecievingCard))))
    (:Is%20Not%20Valid
      (return true))))

(fn ConditionifPlayerHasCardsinGraveyard
  (params (Controller :type Controller%20Object%20Reference) (AI%20Only :type Boolean) (MinCardsInGraveyard :type Integer))
  (if AI%20Only
    (if (.Valid (CallFunction|GetAiControllerReference(ServerOnly) Controller))
      _
      (else
        (return true))))
  (return (>= (Utilities|Array|Length (Variables|/Game/WoW_TCG/Blueprints/Gameplay/Graveyard.Graveyard_C|GetGraveyardList (Default|GetGraveyardReference (.AsTCG%20Game%20State (Utilities|Casting|CastToTCG_GameState (Game|GetGameState))) (CallFunction|GetControllerID(ServerOnly) Controller)))) MinCardsInGraveyard)))

(fn ConditionifLowPlayableCardsinHand(AIOnly)
  (params (PlayerID :type Integer) (LowValue :type Integer))
  (if false
    (return (<= (Utilities|Array|Length (Variables|/Game/WoW_TCG/TCG_AI/AI_Blueprint/TCG_AI_Controller.TCG_AI_Controller_C|GetPlayable%20Cards%20In%20Hand%20List (.TCG%20AI%20Controller (CallFunction|GetAiControllerReference(ServerOnly) (CallFunction|GetControllerReferencefromID(ServerOnly) PlayerID))))) LowValue))
    (else
      (return true))))