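; Function library that computes widget transforms to lay out a player's hand of cards in the card game.
; Fanned centers on the current card count, optionally tightening spacing as the hand fills.
; Horizontale centers on maximum hand size with fixed spacing, leaving its dynamic-spacing calculation unconnected.
; Both turn offset from center into position, parabolic arc and optional linear tilt, with scaling, screen offsets and direction mirroring.
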(fn Fanned
  (params (Card%20Widget%20Reference :type Widget%20Object%20Reference) (Card%20Loop%20Index :type Integer) (Cards%20In%20Hand :type Integer) (Max%20Cards%20In%20Hand :type Integer) (Screen%20Resolution :type Vector%202D%20Structure) (Card%20Size :type Vector%202D%20Structure) (Fly%20In%20Direction :type Boolean) (Rotate%20Cards%20To%20Offset :type Boolean) (Card%20Offset :type Float%20%28single-precision%29) (Rotation%20Distance%20Scale%20Factor :type Float%20%28single-precision%29) (RadiusOffset :type Float%20%28single-precision%29) (Card%20Spacing%20%28Min%29 :type Float%20%28single-precision%29) (Dynamic%20Spacing :type Boolean) (Dynamic%20Spacing%20Max%20Offset :type Float%20%28single-precision%29) (Screen%20Offset%20X :type Float%20%28single-precision%29) (Screen%20Offset%20Y :type Float%20%28single-precision%29) (Viewport%20Scale :type Float%20%28single-precision%29) (Card%20Scale :type Float%20%28single-precision%29))
  (bind _returnvalue (Math|Conversions|ToFloat(Integer) Max%20Cards%20In%20Hand))
  (bind _returnvalue_2 (Math|Conversions|ToFloat(Integer) Cards%20In%20Hand))
  (bind _returnvalue_3 (Math|Conversions|ToFloat(Integer) Card%20Loop%20Index))
  (bind _returnvalue_4 (- Cards%20In%20Hand 1))
  (bind _returnvalue_5 (* Rotation%20Distance%20Scale%20Factor 2e+01))
  (bind _returnvalue_6 (/ _returnvalue_2 _returnvalue))
  (bind _returnvalue_7 (Math|Conversions|ToFloat(Integer) _returnvalue_4))
  (bind _returnvalue_8 (Math|Float|Lerp Dynamic%20Spacing%20Max%20Offset Card%20Spacing%20%28Min%29 _returnvalue_6))
  (bind _returnvalue_9 (/ _returnvalue_7 2.0))
  (bind _returnvalue_10 (Math|Float|Clamp(Float) _returnvalue_8 Card%20Spacing%20%28Min%29 Dynamic%20Spacing%20Max%20Offset))
  (bind _returnvalue_11 (+ _returnvalue_9 Card%20Offset))
  (bind _returnvalue_12 (- _returnvalue_3 _returnvalue_11))
  (bind _returnvalue_13 (select Dynamic%20Spacing _returnvalue_10 Card%20Spacing%20%28Min%29))
  (bind _returnvalue_14 (* _returnvalue_12 _returnvalue_5))
  (bind _returnvalue_15 (* _returnvalue_12 _returnvalue_13))
  (bind _returnvalue_16 (* _returnvalue_14 -1.0))
  (return (Utilities|Struct|MakeWidgetTransform (Math|Vector2D|MakeVector2D (+ Screen%20Offset%20X (* (select Fly%20In%20Direction _returnvalue_15 (* _returnvalue_15 -1.0)) Card%20Scale)) (* (- (* (* _returnvalue_12 (* _returnvalue_15 RadiusOffset)) -1.0) Screen%20Offset%20Y) Card%20Scale)) (Math|Vector2D|MakeVector2D Card%20Scale Card%20Scale) (* (select Rotate%20Cards%20To%20Offset (select (>= _returnvalue_3 _returnvalue_11) (select Fly%20In%20Direction _returnvalue_16 _returnvalue_14) (select Fly%20In%20Direction _returnvalue_16 _returnvalue_14)) 0.0) -1.0))))

(fn Horizontale
  (params (Card%20Widget%20Reference :type Widget%20Object%20Reference) (Card%20Loop%20Index :type Integer) (Cards%20In%20Hand :type Integer) (Max%20Cards%20In%20Hand :type Integer) (Screen%20Resolution :type Vector%202D%20Structure) (Card%20Size :type Vector%202D%20Structure) (Fly%20In%20Direction :type Boolean) (Rotate%20Cards%20To%20Offset :type Boolean) (RadiusOffset :type Float%20%28single-precision%29) (Rotation%20Distance%20Scale%20Factor :type Float%20%28single-precision%29) (Card%20Spacing :type Float%20%28single-precision%29) (Dynamic%20Spacing :type Boolean) (Card%20Spacing%20Max :type Float%20%28single-precision%29) (Screen%20Offset%20X :type Float%20%28single-precision%29) (Card%20Scale :type Float%20%28single-precision%29) (Viewport%20Scale :type Float%20%28single-precision%29) (Screen%20Offset%20Y :type Float%20%28single-precision%29) (Card%20Offset :type Float%20%28single-precision%29))
  (bind _returnvalue (Math|Conversions|ToFloat(Integer) Card%20Loop%20Index))
  (bind _returnvalue_2 (- Max%20Cards%20In%20Hand 1))
  (bind _returnvalue_3 (* Rotation%20Distance%20Scale%20Factor 2e+01))
  (bind _returnvalue_4 (Math|Conversions|ToFloat(Integer) _returnvalue_2))
  (bind _returnvalue_5 (/ _returnvalue_4 2.0))
  (bind _returnvalue_6 (+ _returnvalue_5 Card%20Offset))
  (bind _returnvalue_7 (- _returnvalue _returnvalue_6))
  (bind _returnvalue_8 (* _returnvalue_7 _returnvalue_3))
  (bind _returnvalue_9 (* _returnvalue_7 Card%20Spacing))
  (bind _returnvalue_10 (- _returnvalue_9 0.0))
  (bind _returnvalue_11 (* _returnvalue_8 -1.0))
  (bind _returnvalue_12 (* _returnvalue_10 Card%20Scale))
  (return (Utilities|Struct|MakeWidgetTransform (Math|Vector2D|MakeVector2D (+ (select Fly%20In%20Direction _returnvalue_12 (* _returnvalue_12 -1.0)) Screen%20Offset%20X) (* (- (+ (* (* _returnvalue_7 (* _returnvalue_9 RadiusOffset)) -1.0) 1.0) Screen%20Offset%20Y) Card%20Scale)) (Math|Vector2D|MakeVector2D Card%20Scale Card%20Scale) "(X=0.000000,Y=0.000000)" (* (select Rotate%20Cards%20To%20Offset (select (>= _returnvalue (Math|Conversions|ToFloat(Integer) Cards%20In%20Hand)) (select Fly%20In%20Direction _returnvalue_11 _returnvalue_8) (select Fly%20In%20Direction _returnvalue_11 _returnvalue_8)) 0.0) -1.0))))